(fn `GetPickupMessage`
  (returns (Text :type Text) (LeftImage :type "Texture2D Object Reference") (RightImage :type "Texture2D Object Reference"))
  (return (`|FormatText` "You picked up the {WeaponName}" (`.ItemName` (defaults `Object` (`self.WeaponClass`)))) null null))

(fn `UserConstructionScript`
  (bind _asshooter_weapon (cast `ShooterWeapon` (`ShooterBlueprintLibrary.GetDefaultObjectFromClass` (`self.WeaponClass`))))
  (`SkinnedMeshComponent.SetSkinnedAssetAndUpdate` (`self.PickupMeshComp`) (`SkinnedMeshComponent.SkeletalMesh` (`ShooterWeapon.Mesh3P` _asshooter_weapon)) true))