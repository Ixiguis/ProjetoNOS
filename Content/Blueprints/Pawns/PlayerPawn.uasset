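; Player pawn Blueprint for a shooter, adding a first-person body, shadows and a blink-teleport target marker.
; Body and shadow meshes copy the main mesh's look and animation, toggle with view mode, and the body follows camera updates.
; While preparing a blink, Tick line-traces from the view to place the marker at the hit, before a character, or at maximum range.
; Weapon events update the shadow weapon mesh and local ammo HUD.
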(event `self.ReceiveTick`
  (params (DeltaSeconds :type "Float (single-precision)"))
  (`parent.ReceiveTick` DeltaSeconds)
  (`self.Update Blink Marker`))

(event `self.SetIsPreparingBlink`
  (params (IsPreparingBlink :type Boolean))
  (bind _blinktarget (`self.BlinkTarget`))
  (`parent.SetIsPreparingBlink` IsPreparingBlink)
  (if (`self.Get Is Preparing Blink`)
    (`SceneComponent.SetHiddenInGame` _blinktarget false false)
    (else
      (`SceneComponent.SetHiddenInGame` _blinktarget true false))))

(event `self.PawnDiedEvent`
  (params (PawnInstigator :type "Pawn Object Reference") (DamageCauser :type "Actor Object Reference"))
  ;[1 1 1] Update first person weapon shadow
  (`parent.PawnDiedEvent` PawnInstigator DamageCauser)
  (`PrimitiveComponent.SetCastShadow` (`self.Mesh1PBodyShadow`) false)
  (`PrimitiveComponent.SetCastShadow` (`self.WeaponMesh1PShadow`) false))

(event `WeaponEquipped` :!signature `self.OnWeaponEquipped`
  (params (WeaponEquipped :type "ShooterWeapon Object Reference"))
  (bind _weaponmesh1pshadow (`self.WeaponMesh1PShadow`))
  ;[1 1 1] Update first person weapon shadow
  (`SkinnedMeshComponent.SetSkinnedAssetAndUpdate` _weaponmesh1pshadow (`SkinnedMeshComponent.SkeletalMesh` (`ShooterWeapon.Mesh3P` WeaponEquipped)) true)
  (`SceneComponent.K2_AttachTo` _weaponmesh1pshadow (`self.Mesh1PBodyShadow`) (`self.WeaponAttachPoint`) "SnapToTarget" true))

(event `self.ReceiveBeginPlay`
  ;[1 1 1] Update first person weapon shadow
  (`parent.ReceiveBeginPlay`)
  (add `self.OnWeaponEquipped` (delegate `WeaponEquipped`)))

(event `self.UpdatePawnMeshes_BP`
  (bind _returnvalue (`self.IsFirstPerson`))
  (bind _mesh1pbody (`self.Mesh1PBody`))
  (bind _mesh1pbodyshadow (`self.Mesh1PBodyShadow`))
  ;[1 1 1] UpdatePawnMeshes
  (`parent.UpdatePawnMeshes_BP`)
  (`SceneComponent.SetHiddenInGame` _mesh1pbody (not _returnvalue) false)
  (`PrimitiveComponent.SetCastShadow` _mesh1pbodyshadow _returnvalue)
  (bind _asshooter_anim_instance (cast `ShooterAnimInstance` (`SkeletalMeshComponent.GetAnimInstance` _mesh1pbody))
    (:`then`
      (set `ShooterAnimInstance.bIsMesh1PBody` true _asshooter_anim_instance)
      (set `ShooterAnimInstance.bProcessAnimNotifies` false _asshooter_anim_instance))
    (:`CastFailed`
      _))
  (bind _asshooter_anim_instance_2 (cast `ShooterAnimInstance` (`SkeletalMeshComponent.GetAnimInstance` _mesh1pbodyshadow))
    (:`then`
      (set `ShooterAnimInstance.bProcessAnimNotifies` false _asshooter_anim_instance_2))
    (:`CastFailed`
      _))
  (if _returnvalue
    (set `SkinnedMeshComponent.VisibilityBasedAnimTickOption` "AlwaysTickPoseAndRefreshBones" (`self.Mesh1PBodyShadow`))
    (set `SkinnedMeshComponent.VisibilityBasedAnimTickOption` "AlwaysTickPoseAndRefreshBones" (`self.Mesh1PBody`))
    (else
      (set `SkinnedMeshComponent.VisibilityBasedAnimTickOption` "OnlyTickPoseWhenRendered" (`self.Mesh1PBodyShadow`))
      (set `SkinnedMeshComponent.VisibilityBasedAnimTickOption` "OnlyTickPoseWhenRendered" (`self.Mesh1PBody`)))))

(event `self.OnCameraUpdate`
  (params (CameraLocation :type "Vector Structure (by ref)") (CameraRotation :type "Rotator Structure (by ref)"))
  ;[1 1 1] Camera update, updates first person body position
  (`parent.OnCameraUpdate` CameraLocation CameraRotation)
  (`SceneComponent.K2_SetRelativeLocation` (`self.Mesh1PBody`) (`KismetMathLibrary.MakeVector` (.x (`KismetMathLibrary.LessLess_VectorRotator` (- CameraLocation (`SceneComponent.GetSocketLocation` (`self.Mesh`) "CameraLocation")) (`KismetMathLibrary.MakeRotator` 0.0 0.0 (+ (.yaw CameraRotation) -90.0)))) (.y (`KismetMathLibrary.LessLess_VectorRotator` (- CameraLocation (`SceneComponent.GetSocketLocation` (`self.Mesh`) "CameraLocation")) (`KismetMathLibrary.MakeRotator` 0.0 0.0 (+ (.yaw CameraRotation) -90.0)))) (- (.z (`KismetMathLibrary.LessLess_VectorRotator` (- CameraLocation (`SceneComponent.GetSocketLocation` (`self.Mesh`) "CameraLocation")) (`KismetMathLibrary.MakeRotator` 0.0 0.0 (+ (.yaw CameraRotation) -90.0)))) (`self.FixedCameraHeight`))) false false))

(event `self.OnWeaponAdded`
  (params (WeaponClass :type "ShooterWeapon Class Reference"))
  ;[1 1 1] (Weapon added) Update weapons HUD
  (bind _asshooter_player_controller_bp (cast `/Game/Blueprints/Game/ShooterPlayerController_BP` (`self.GetController`)))
  (if (`Controller.IsLocalPlayerController` _asshooter_player_controller_bp)
    (`/Game/Blueprints/Game/ShooterPlayerController_BP.Add Weapon Ammo HUD` _asshooter_player_controller_bp WeaponClass)))

(fn `UserConstructionScript`
  (bind _mesh (`self.Mesh`))
  (`parent.UserConstructionScript`)
  (`SkinnedMeshComponent.SetSkinnedAssetAndUpdate` (`self.Mesh1PBodyShadow`) (`SkinnedMeshComponent.SkeletalMesh` _mesh) true)
  (`SkinnedMeshComponent.SetSkinnedAssetAndUpdate` (`self.Mesh1PBody`) (`SkinnedMeshComponent.SkeletalMesh` _mesh) true) ; Copy SkeletalMesh from "Mesh"
  (for _index (range (`PrimitiveComponent.GetNumMaterials` (`self.Mesh1PBodyShadow`)))
    (`PrimitiveComponent.SetMaterial` (`self.Mesh1PBody`) _index (`PrimitiveComponent.GetMaterial` _mesh _index))
    (`PrimitiveComponent.SetMaterial` (`self.Mesh1PBodyShadow`) _index (`PrimitiveComponent.GetMaterial` _mesh _index)) ; Copy materials from "Mesh"
  )
  (`SkeletalMeshComponent.SetAnimInstanceClass` (`self.Mesh1PBodyShadow`) (`GameplayStatics.GetObjectClass` (`SkeletalMeshComponent.GetAnimInstance` _mesh)))
  (`SkeletalMeshComponent.SetAnimInstanceClass` (`self.Mesh1PBody`) (`GameplayStatics.GetObjectClass` (`SkeletalMeshComponent.GetAnimInstance` _mesh))) ; Copy AnimInstance from "Mesh"
)