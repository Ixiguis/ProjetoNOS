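; Alien pawn that steadily loses health unless it keeps landing damaging kicks on shooter characters.
; On the authority, Tick applies environmental damage per second to itself once the time since the last damage timestamp exceeds a set delay.
; The timestamp starts at construction, and the ProcessKick override resets it when a kick deals damage and the kicked character's health remains above zero.
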(event `self.ReceiveTick`
  (params (DeltaSeconds :type "Float (single-precision)"))
  (`parent.ReceiveTick` DeltaSeconds)
  (`/Engine/EditorBlueprintResources/ActorMacros.Switch Has Authority`
    (:`Authority`
      (if (> (- (`KismetSystemLibrary.GetGameTimeInSeconds`) (`self.LastDamageTime`)) (`self.StartDamageAfter`))
        (`GameplayStatics.ApplyDamage` self (* DeltaSeconds (`self.SelfDamageDPS`)) (`self.GetController`) self "/Game/Blueprints/DamageTypes/DmgType_ShooterEnvironmental.DmgType_ShooterEnvironmental_C")))))

(event `KickedSomeone`
  (params (KickedActor :type "Actor Object Reference") (DamageDealt :type "Float (double-precision)")))

(fn `ProcessKick`
  (returns (DamageDealt :type "Float (double-precision)") (KickedActor :type "Actor Object Reference"))
  (bind (_damagedealt _kickedactor) (`parent.ProcessKick`))
  (bind _asshooter_character (cast `ShooterCharacter` _kickedactor)
    (:`then`
      (if (and (> (`ShooterCharacter.Health` _asshooter_character) 0.0) (> _damagedealt 0.0))
        (set `self.LastDamageTime` (`KismetSystemLibrary.GetGameTimeInSeconds`))))
    (:`CastFailed`
      _))
  (return _damagedealt _kickedactor))

(fn `UserConstructionScript`
  (`parent.UserConstructionScript`)
  (set `self.LastDamageTime` (`KismetSystemLibrary.GetGameTimeInSeconds`)))