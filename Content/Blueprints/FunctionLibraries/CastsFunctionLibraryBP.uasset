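; Blueprint function library of shortcut getters for the shooter game's core framework objects.
; Separate functions fetch the current Game Instance, Game State and Game Mode and cast each to its project-specific shooter class.
; Each returns the typed cast result directly, with no additional handling of a failed cast.
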(fn `Get Shooter Game Instance`
  (returns (`AsShooter Game Instance BP` :type "/Game/Blueprints/Game/ShooterGameInstance_BP Object Reference"))
  (return (cast `/Game/Blueprints/Game/ShooterGameInstance_BP` (`GameplayStatics.GetGameInstance` null) :!pure true)))

(fn `Get Shooter Game Mode`
  (returns (`AsShooter Game Mode` :type "ShooterGameMode Object Reference"))
  (return (cast `ShooterGameMode` (`GameplayStatics.GetGameMode` null) :!pure true)))

(fn `Get Shooter Game State`
  (returns (`AsShooter Game State` :type "ShooterGameState Object Reference"))
  (return (cast `ShooterGameState` (`GameplayStatics.GetGameState` null) :!pure true)))