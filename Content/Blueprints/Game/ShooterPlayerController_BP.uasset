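; Shooter player controller that owns the local player's UI: main HUD, scoreboard, menu shortcuts and a radial weapon-selection menu.
; A macro lazily creates the HUD for local controllers, fed by possession, ammo, pickup and game-state events.
; Held category keys open a data-table-driven radial menu of owned weapons, zeroing mouse sensitivity until release equips the selection.
; The scoreboard refreshes on player join or leave and takes over next/previous-weapon input for scrolling.
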(event `self.Possessed`
  (params (NewPawn :type "Pawn Object Reference"))
  (`self.Update Player Character` :!label _label))

(event `self.OnPlayerStateReplicated`
  (goto _label))

(event `self.NotifyGameEnded`
  (`self.Destroy HUD` :!label _label_2))

(event `self.ReceiveDestroyed`
  (`|ExecutionSequence`
    (:`then_0`
      (goto _label_2))
    (:`then_1`
      (`parent.ReceiveDestroyed`))))

(event `InputAction|InGameMenu`
  (params (Key :type "Key Structure"))
  ;[1 1 1] Open menus
  (:`Pressed`
    (`/Game/Blueprints/Game/ShooterGameInstance_BP.OpenInGameMenu` (cast `/Game/Blueprints/Game/ShooterGameInstance_BP` (`GameplayStatics.GetGameInstance`) :!pure true))))

(event `InputAction|DebugOpenMainMenu`
  (params (Key :type "Key Structure"))
  ;[1 1 1] Open menus
  (:`Pressed`
    (`/Game/Blueprints/Game/ShooterGameInstance_BP.GoToMainMenu` (cast `/Game/Blueprints/Game/ShooterGameInstance_BP` (`GameplayStatics.GetGameInstance`) :!pure true))))

(event `InputAction|WeaponCat1`
  (params (Key :type "Key Structure"))
  ;[1 1 1] Switch weapons
  (:`Pressed`
    (if (not (`self.Is Radial Menu Open`))
      (set `self.Selected weapon category row name` "Category1")
      (`self.Open Weapon Selection` :!label _label_3)))
  (:`Released`
    (`self.Close Radial Menu` :!label _label_4)))

(event `InputAction|WeaponCat2`
  (params (Key :type "Key Structure"))
  ;[1 1 1] Switch weapons
  (:`Pressed`
    (if (not (`self.Is Radial Menu Open`))
      (set `self.Selected weapon category row name` "Category2")
      (goto _label_3)))
  (:`Released`
    (goto _label_4)))

(event `InputAction|WeaponCat3`
  (params (Key :type "Key Structure"))
  ;[1 1 1] Switch weapons
  (:`Pressed`
    (if (not (`self.Is Radial Menu Open`))
      (set `self.Selected weapon category row name` "Category3")
      (goto _label_3)))
  (:`Released`
    (goto _label_4)))

(event `InputAction|ToggleScoreboard`
  (params (Key :type "Key Structure"))
  (:`Pressed`
    (`/Engine/EditorBlueprintResources/StandardMacros.FlipFlop`
      (:`A`
        (`self.Open Scoreboard`))
      (:`B`
        (`self.Close Scoreboard`)))))

(event `InputAction|PeekScoreboard`
  (params (Key :type "Key Structure"))
  (:`Pressed`
    (`self.Open Scoreboard`))
  (:`Released`
    (`self.Close Scoreboard`)))

(event `InputAction|NextWeapon` :consume false
  (params (Key :type "Key Structure"))
  (bind _scoreboard_widget_ref (`self.Scoreboard Widget Ref`))
  (:`Pressed`
    (`/Engine/EditorBlueprintResources/StandardMacros.IsValid` _scoreboard_widget_ref
      (:`Is Valid`
        (`/Game/UI/Widgets/Scoreboard/Scoreboard.Scroll Up` _scoreboard_widget_ref)))))

(event `InputAction|PrevWeapon` :consume false
  (params (Key :type "Key Structure"))
  (bind _scoreboard_widget_ref (`self.Scoreboard Widget Ref`))
  (:`Pressed`
    (`/Engine/EditorBlueprintResources/StandardMacros.IsValid` _scoreboard_widget_ref
      (:`Is Valid`
        (`/Game/UI/Widgets/Scoreboard/Scoreboard.Scroll down` _scoreboard_widget_ref)))))

(event `self.NotifyPlayerJoinedGame`
  (params (NewPlayerState :type "PlayerState Object Reference"))
  (`self.Update Scoreboard If Open` :!label _label))

(event `self.NotifyPlayerLeftGame`
  (params (LeavingPlayerState :type "PlayerState Object Reference"))
  (goto _label))

(event `On Radial Menu Selection`
  (params (`Selected Option` :type "/Game/Blueprints/Enums/RadialMenuOptions Enum" :default "NewEnumerator0"))
  (if (`|EnumInequality` `Selected Option` "NewEnumerator0")
    (bind _returnvalue (`|GetDataTableRow` "/Game/Blueprints/DataTables/RadialMenuWeaponOptions.RadialMenuWeaponOptions" (`self.Selected weapon category row name`))
      (:`then`
        (bind ((`TopItem_14_D5DE697A4F9C9789C1FF4381E099B2A7` _topitem) (`BottomItem_15_F34480814F59D11F60CAF9A0943B58BD` _bottomitem) (`LeftItem_16_22A18AAA46929162912DC783C411FF19` _leftitem) (`RightItem_17_FEEDB1764B77212F524E28A2D65D5A5D` _rightitem)) (break `/Game/Blueprints/DataTables/RadialMenuItemSelection` _returnvalue))
        (`ShooterCharacter.EquipItemByClass` (`self.My ShooterCharacter`) (select `/Game/Blueprints/Enums/RadialMenuOptions` `Selected Option` :`NewEnumerator1` _topitem :`NewEnumerator2` _bottomitem :`NewEnumerator3` _leftitem :`NewEnumerator4` _rightitem))))))

(event `self.CrosshairChanged`
  (params (NewCrosshair :type "Texture2D Object Reference"))
  (`/Game/UI/Widgets/HUDMain.SetCrosshair` (`self.HUDMain Widget Ref`) NewCrosshair))

(event `Add Weapon Ammo HUD`
  (params (`Weapon Class` :type "ShooterWeapon Class Reference (by ref)"))
  (bind _hudmainref (`self.Conditional Create HUD`)
    (:`HUD Valid`
      (`/Game/UI/Widgets/HUDMain.Add Weapon` _hudmainref `Weapon Class`))))

(event `self.GameModeAndStateInitialized`
  (bind _hudmainref (`self.Conditional Create HUD`)
    (:`HUD Valid`
      (`/Game/UI/Widgets/HUDMain.Update GameState` _hudmainref))))

(event `self.NotifyPickup`
  (params (Pickup :type "ShooterPickup Object Reference"))
  (bind _hudmainref (`self.Conditional Create HUD`)
    (:`HUD Valid`
      (`/Game/UI/Widgets/HUDMain.Add text to bottom center` _hudmainref (`ShooterPickup.GetPickupMessage` Pickup) false))))

(fn `Close Radial Menu`
  (bind _saved_mousesensitivity (`self.Saved MouseSensitivity`))
  (if (`self.Is Radial Menu Open`)
    (`self.On Radial Menu Selection` (`/Game/UI/Widgets/RadialMenu.Current Option` (`self.RadialMenu Widget Ref`)))
    (`Widget.RemoveFromParent` (`self.RadialMenu Widget Ref`))
    (`self.SetMouseSensitivityX` _saved_mousesensitivity)
    (`self.SetMouseSensitivityY` _saved_mousesensitivity)
    (set `self.Is Radial Menu Open` false)))

(fn `Close Scoreboard`
  (bind _my_shootercharacter (`self.My ShooterCharacter`))
  (`/Engine/EditorBlueprintResources/StandardMacros.IsValid` (`self.Scoreboard Widget Ref`)
    (:`Is Valid`
      (`Widget.RemoveFromParent` (`self.Scoreboard Widget Ref`)))
    (:`Is Not Valid`
      _))
  (`/Engine/EditorBlueprintResources/StandardMacros.IsValid` _my_shootercharacter
    (:`Is Valid`
      (`ShooterCharacter.SetPrevNextWeaponEventEnabled` _my_shootercharacter true))))

(fn `Destroy HUD`
  (bind _hudmain_widget_ref (`self.HUDMain Widget Ref`))
  (`/Engine/EditorBlueprintResources/StandardMacros.IsValid` _hudmain_widget_ref
    (:`Is Valid`
      (`Widget.RemoveFromParent` _hudmain_widget_ref)
      (`/Game/UI/Widgets/HUDMain.Destroy` _hudmain_widget_ref))))

(fn `Open Scoreboard`
  (bind _my_shootercharacter (`self.My ShooterCharacter`))
  (`/Engine/EditorBlueprintResources/StandardMacros.IsValid` (`self.Scoreboard Widget Ref`)
    (:`Is Valid`
      _)
    (:`Is Not Valid`
      (bind _returnvalue (`|CreateWidget` "/Game/UI/Widgets/Scoreboard/Scoreboard.Scoreboard_C" self))
      (set `self.Scoreboard Widget Ref` _returnvalue)))
  (`UserWidget.AddToViewport` (`self.Scoreboard Widget Ref`) 0)
  (`/Game/UI/Widgets/Scoreboard/Scoreboard.Update Scoreboard` (`self.Scoreboard Widget Ref`))
  (`/Engine/EditorBlueprintResources/StandardMacros.IsValid` _my_shootercharacter
    (:`Is Valid`
      (`ShooterCharacter.SetPrevNextWeaponEventEnabled` _my_shootercharacter false))))

(fn `Open Weapon Selection`
  (bind _my_shootercharacter (`self.My ShooterCharacter`))
  (bind _returnvalue (`|GetDataTableRow` "/Game/Blueprints/DataTables/RadialMenuWeaponOptions.RadialMenuWeaponOptions" (`self.Selected weapon category row name`))
    (:`then`
      (bind (_topitem _bottomitem _leftitem _rightitem _backgroundcolor _selectioncolor) (break `/Game/Blueprints/DataTables/RadialMenuItemSelection` _returnvalue))
      (`self.Show Radial Menu` (select `bool` (`KismetSystemLibrary.IsValid` (`ShooterCharacter.FindItem` _my_shootercharacter _topitem)) :`true` (defaults `Object` _topitem)) (select `bool` (`KismetSystemLibrary.IsValid` (`ShooterCharacter.FindItem` _my_shootercharacter _bottomitem)) :`true` (defaults `Object` _bottomitem)) (select `bool` (`KismetSystemLibrary.IsValid` (`ShooterCharacter.FindItem` _my_shootercharacter _leftitem)) :`true` (defaults `Object` _leftitem)) (select `bool` (`KismetSystemLibrary.IsValid` (`ShooterCharacter.FindItem` _my_shootercharacter _rightitem)) :`true` (defaults `Object` _rightitem)) _backgroundcolor _selectioncolor))))

(fn `Show Radial Menu`
  (params (`Top Texture` :type "Texture2D Object Reference") (`Bottom Texture` :type "Texture2D Object Reference") (`Left Texture` :type "Texture2D Object Reference") (`Right Texture` :type "Texture2D Object Reference") (`Background Color` :type "LinearColor Structure") (`Selection Color` :type "LinearColor Structure"))
  (bind _radialmenu_widget_ref (`self.RadialMenu Widget Ref`))
  (if (or (`KismetSystemLibrary.IsValid` `Top Texture`) (`KismetSystemLibrary.IsValid` `Bottom Texture`) (`KismetSystemLibrary.IsValid` `Left Texture`) (`KismetSystemLibrary.IsValid` `Right Texture`))
    (`/Engine/EditorBlueprintResources/StandardMacros.IsValid` (`self.RadialMenu Widget Ref`)
      (:`Is Valid`
        (`/Game/UI/Widgets/RadialMenu.Set Radial Menu Properties` _radialmenu_widget_ref `Selection Color` `Background Color` `Top Texture` `Bottom Texture` `Left Texture` `Right Texture` :!label _label)
        (`UserWidget.AddToViewport` _radialmenu_widget_ref 0)
        (set `self.Saved MouseSensitivity` (`self.GetMouseSensitivityX`))
        (set `self.Is Radial Menu Open` true)
        (`self.SetMousePositionToCenter`)
        (`self.SetMouseSensitivityX` 0.0)
        (`self.SetMouseSensitivityY` 0.0))
      (:`Is Not Valid`
        (if (`self.IsLocalPlayerController`)
          (bind _returnvalue (`|CreateWidget` "/Game/UI/Widgets/RadialMenu.RadialMenu_C" self))
          (set `self.RadialMenu Widget Ref` _returnvalue)
          (goto _label))))))

(fn `Update Player Character`
  (bind _asshooter_character_bp (cast `/Game/Blueprints/Pawns/ShooterCharacter_BP` (`self.K2_GetPawn`)))
  (set `self.My ShooterCharacter` _asshooter_character_bp)
  (bind _hudmainref (`self.Conditional Create HUD`)
    (:`HUD Valid`
      (`/Game/UI/Widgets/HUDMain.Update Player Character` _hudmainref (`self.My ShooterCharacter`) self))))

(fn `Update Scoreboard If Open`
  (`/Engine/EditorBlueprintResources/StandardMacros.IsValid` (`self.Scoreboard Widget Ref`)
    (:`Is Valid`
      (if (`Widget.IsInViewport` (`self.Scoreboard Widget Ref`))
        (`/Game/UI/Widgets/Scoreboard/Scoreboard.Update Scoreboard` (`self.Scoreboard Widget Ref`))))))

(fn `UserConstructionScript`
  (`parent.UserConstructionScript`))