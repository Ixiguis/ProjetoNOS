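; Tutorial map HUD that draws centered text messages in the upper part of the screen.
; Temporary messages show in white for a set duration, with alpha fading in and out from elapsed game time.
; A persistent red message fades in and shows whenever no temporary message is active, until it is removed.
; Other code drives it through functions that store the text and timestamp, which DrawHUD reads each frame.
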(event `self.ReceiveDrawHUD`
  (params (SizeX :type Integer) (SizeY :type Integer))
  (bind _scaleui (`self.ScaleUI`))
  (bind _tempmessageduration (`self.TempMessageDuration`))
  (bind _persistentmessagetodraw (`self.PersistentMessageToDraw`))
  (bind _scaleui_2 (`self.ScaleUI`))
  (bind _returnvalue (/ _tempmessageduration 2.0))
  (bind _returnvalue_2 (* (`self.HudSizeY`) 0.3))
  (bind _returnvalue_3 (- (`KismetSystemLibrary.GetGameTimeInSeconds`) (`self.TempMessageAddedTime`)))
  (set `self.HudSizeX` SizeX)
  (set `self.HudSizeY` SizeY)
  (if (<= _returnvalue_3 _tempmessageduration)
    (`self.DrawText` (`self.TempMessageToDraw`) (make `LinearColor` 1.0 1.0 1.0 (`KismetMathLibrary.FClamp` (* (- _returnvalue (`KismetMathLibrary.Abs` (- _returnvalue_3 _returnvalue))) 2.0))) (- (`KismetMathLibrary.Conv_IntToDouble` (/ (`self.HudSizeX`) 2)) (/ (`self.GetTextSize` (`self.TempMessageToDraw`) "/Game/UI/HUD/Roboto51.Roboto51" _scaleui) 2.0)) _returnvalue_2 "/Game/UI/HUD/Roboto51.Roboto51" _scaleui)
    (elif (`KismetStringLibrary.NotEqual_StrStr` _persistentmessagetodraw)
      (`self.DrawText` _persistentmessagetodraw (make `LinearColor` 1.0 0.1 0.1 (`KismetMathLibrary.FClamp` (* (- (`KismetSystemLibrary.GetGameTimeInSeconds`) (`self.PersistentMessageAddedTime`)) 2.0))) (- (`KismetMathLibrary.Conv_IntToDouble` (/ (`self.HudSizeX`) 2)) (/ (`self.GetTextSize` _persistentmessagetodraw "/Game/UI/HUD/Roboto51.Roboto51" _scaleui_2) 2.0)) _returnvalue_2 "/Game/UI/HUD/Roboto51.Roboto51" _scaleui_2))))

(fn `AddPersistentMessage`
  (params (Message :type Text))
  (set `self.PersistentMessageToDraw` (`KismetTextLibrary.Conv_TextToString` Message))
  (set `self.PersistentMessageAddedTime` (`KismetSystemLibrary.GetGameTimeInSeconds`)))

(fn `AddTemporaryMessage`
  (params (Message :type Text) (Duration :type "Float (double-precision)"))
  (set `self.TempMessageToDraw` (`KismetTextLibrary.Conv_TextToString` Message))
  (set `self.TempMessageDuration` Duration)
  (set `self.TempMessageAddedTime` (`KismetSystemLibrary.GetGameTimeInSeconds`)))

(fn `RemovePersistentMessage`
  (set `self.PersistentMessageToDraw` ""))

(fn `UserConstructionScript`)