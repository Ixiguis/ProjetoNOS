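; Light01 is an environment light fixture Blueprint that pairs a spot light with a static mesh whose material color matches the light.
; The construction script applies the radius, intensity and color variables to the spot light and creates a dynamic material instance on the mesh's second material slot, setting its Color parameter.
; ChangeLightColor updates both the spot light and that stored material instance, keeping them in sync.
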(fn `ChangeLightColor`
  (params (NewColor :type "LinearColor Structure"))
  (`LightComponent.SetLightColor` (`self.SpotLight1`) NewColor true)
  (`MaterialInstanceDynamic.SetVectorParameterValue` (`self.LightMID`) "Color" NewColor))

(fn `UserConstructionScript`
  (bind _spotlight1 (`self.SpotLight1`))
  (`PointLightComponent.SetAttenuationRadius` _spotlight1 (`self.LightRadius`))
  (`LightComponent.SetIntensity` _spotlight1 (`self.LightIntensity`))
  (`LightComponent.SetLightColor` _spotlight1 (`self.LightColor`) true)
  (bind _returnvalue (`PrimitiveComponent.CreateDynamicMaterialInstance` (`self.StaticMesh`) 1 null))
  (set `self.LightMID` _returnvalue)
  (`MaterialInstanceDynamic.SetVectorParameterValue` _returnvalue "Color" (`self.LightColor`)))