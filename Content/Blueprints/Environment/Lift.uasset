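; Lift actor that makes a timed round trip when something overlaps its trigger volume.
; A timeline lerps the mesh from start to end, waits, then reverses, with start, loop and end sounds; a DoOnce blocks retriggering until it returns.
; The construction script captures the start position, sets play rate as the inverse of LiftSpeed, applies mesh and material overrides, and snap-attaches listed actors to the mesh.
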(event `self.TriggerVolume.OnComponentBeginOverlap`
  (params (OverlappedComponent :type "PrimitiveComponent Object Reference") (OtherActor :type "Actor Object Reference") (OtherComp :type "PrimitiveComponent Object Reference") (OtherBodyIndex :type Integer) (bFromSweep :type Boolean) (SweepResult :type "HitResult Structure (by ref)"))
  (bind _liftloopsndcomp (`self.LiftLoopSndComp`))
  (bind _liftloopsndcomp_2 (`self.LiftLoopSndComp`))
  (bind _liftloopsndcomp_3 (`self.LiftLoopSndComp`))
  (`/Engine/EditorBlueprintResources/StandardMacros.DoOnce` false :!label _label
    (:`Completed`
      (`KismetSystemLibrary.Delay` (`self.StartMovingDelay`))
      (`GameplayStatics.SpawnSoundAttached` (`self.LiftStartSound`) _liftloopsndcomp_3 "None" (0.0 0.0 0.0) (struct) "EAttachLocation::KeepRelativeOffset")
      (`AudioComponent.Play` _liftloopsndcomp_3 0.0)
      (bind (_direction _newtrack_0) (`Timeline|Timeline - Lift Driver` :!label _label_2)
        (:`Update`
          (`SceneComponent.K2_SetRelativeLocation` (`self.LiftMesh`) (`KismetMathLibrary.VLerp` (`self.LiftStart`) (`self.LiftEnd`) _newtrack_0) false false))
        (:`Finished`
          (`GameplayStatics.SpawnSoundAttached` (`self.LiftEndSound`) _liftloopsndcomp_2 "None" (0.0 0.0 0.0) (struct) "EAttachLocation::KeepRelativeOffset")
          (`AudioComponent.Stop` _liftloopsndcomp_2)
          (switch `ETimelineDirection` _direction
            (:`Forward`
              (`KismetSystemLibrary.RetriggerableDelay` (`self.StayTime`))
              (`GameplayStatics.SpawnSoundAttached` (`self.LiftStartSound`) _liftloopsndcomp "None" (0.0 0.0 0.0) (struct) "EAttachLocation::KeepRelativeOffset")
              (`AudioComponent.Play` _liftloopsndcomp 0.0)
              (goto _label_2 :!via `Reverse`))
            (:`Backward`
              (goto _label :!via `Reset`))))))))

(event `self.LiftMesh.OnComponentHit`
  (params (HitComponent :type "PrimitiveComponent Object Reference") (OtherActor :type "Actor Object Reference") (OtherComp :type "PrimitiveComponent Object Reference") (NormalImpulse :type "Vector Structure") (Hit :type "HitResult Structure (by ref)")))

(fn `UserConstructionScript`
  (bind _material_override (`self.Material Override`))
  (bind _liftloopsndcomp (`self.LiftLoopSndComp`))
  (set `AudioComponent.Sound` (`self.LiftLoopSound`) _liftloopsndcomp)
  (`AudioComponent.Stop` _liftloopsndcomp)
  (`TimelineComponent.SetPlayRate` (`self.Timeline - Lift Driver`) (/ 1.0 (`self.LiftSpeed`)))
  (set `self.LiftStart` (`SceneComponent.RelativeLocation` (`self.LiftMesh`)))
  (`|ExecutionSequence`
    (:`then_0`
      (if (!= (`self.Lift Mesh Override`) null)
        (`StaticMeshComponent.SetStaticMesh` (`self.LiftMesh`) (`self.Lift Mesh Override`))))
    (:`then_1`
      (if (!= _material_override null)
        (`PrimitiveComponent.SetMaterial` (`self.LiftMesh`) 0 _material_override)))
    (:`then_2`
      (for _array_element (`self.AttachActors`)
        (`self.K2_AttachRootComponentTo` _array_element (`self.LiftMesh`) "None" "SnapToTarget" true)))))