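; Physics prop for telekinesis that damages actors it hits while a last grabber is set, crediting that character as instigator.
; Point damage scales with the object's mass, its speed and the relative impact speed, throttled per victim by parallel actor and timestamp arrays.
; Damage from a shooter character while the object moves transfers credit to that character.
; Tick clears the grabber and hit history once the ungrabbed object comes nearly to rest.
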(event `self.ReceiveAnyDamage`
  (params (Damage :type "Float (single-precision)") (DamageType :type "DamageType Object Reference") (InstigatedBy :type "Controller Object Reference") (DamageCauser :type "Actor Object Reference"))
  (`/Engine/EditorBlueprintResources/StandardMacros.IsValid` InstigatedBy
    (:`Is Valid`
      (if (> (`KismetMathLibrary.VSizeSquared` (`SceneComponent.GetComponentVelocity` (`self.StaticMeshComponent`))) 100.0)
        (bind _asshooter_character_bp (cast `/Game/Blueprints/Pawns/ShooterCharacter_BP` (`Controller.K2_GetPawn` InstigatedBy)))
        (`self.SetLastGrabber` _asshooter_character_bp)))))

(event `self.ReceiveTick`
  (params (DeltaSeconds :type "Float (single-precision)"))
  ;[1 1 1] If object stops moving, stop tracking damage
  (if (and (not (`self.IsBeingGrabbed`)) (`KismetSystemLibrary.IsValid` (`self.LastGrabber`)) (`KismetMathLibrary.NearlyEqual_FloatFloat` (`KismetMathLibrary.VSizeSquared` (`self.GetVelocity`)) 0.0 10.0))
    (`self.SetLastGrabber` null)
    (`KismetArrayLibrary.Array_Clear` (`self.DamagedActors`))
    (`KismetArrayLibrary.Array_Clear` (`self.DamagedActorsTime`))))

(event `self.StaticMeshComponent.OnComponentHit`
  (params (HitComponent :type "PrimitiveComponent Object Reference") (OtherActor :type "Actor Object Reference") (OtherComp :type "PrimitiveComponent Object Reference") (NormalImpulse :type "Vector Structure") (Hit :type "HitResult Structure (by ref)"))
  (bind _staticmeshcomponent (`self.StaticMeshComponent`))
  (bind _returnvalue (`KismetArrayLibrary.Array_Find` (`self.DamagedActors`) (`self.Hit actor`)))
  (bind _returnvalue_2 (`SceneComponent.GetComponentVelocity` _staticmeshcomponent))
  (`/Engine/EditorBlueprintResources/StandardMacros.IsValid` OtherActor
    (:`Is Valid`
      (`/Engine/EditorBlueprintResources/StandardMacros.IsValid` (`self.LastGrabber`)
        (:`Is Valid`
          (set `self.Hit actor` OtherActor)
          (`|ExecutionSequence`
            (:`then_0`
              (if (== _returnvalue -1)
                (`KismetArrayLibrary.Array_Add` (`self.DamagedActors`) (`self.Hit actor`))
                (`KismetArrayLibrary.Array_Add` (`self.DamagedActorsTime`) (`KismetSystemLibrary.GetGameTimeInSeconds`))
                (set `self.Can apply damage` true)
                (elif (< (- (`KismetSystemLibrary.GetGameTimeInSeconds`) (`|GetArrayItem` (`self.DamagedActorsTime`) _returnvalue)) (`self.MinDamageInterval`))
                  (set `self.Can apply damage` false)
                  (else
                    (`KismetArrayLibrary.Array_Set` (`self.DamagedActorsTime`) _returnvalue (`KismetSystemLibrary.GetGameTimeInSeconds`))
                    (set `self.Can apply damage` true)))))
            (:`then_1`
              (if (`self.Can apply damage`)
                (`GameplayStatics.ApplyPointDamage` (`self.Hit actor`) (* (* (`KismetMathLibrary.VSize` (- (`self.GetVelocity` (`self.Hit actor`)) _returnvalue_2)) (`KismetMathLibrary.VSize` _returnvalue_2) (`PrimitiveComponent.GetMass` _staticmeshcomponent)) (`self.DamagePerMassPerVelocity`)) (`KismetMathLibrary.Normal` _returnvalue_2) Hit (`Pawn.GetController` (`self.LastGrabber`)) self "/Script/Engine.DamageType")))))))))

(fn `SetLastGrabber`
  (params (`Last Grabber` :type "/Game/Blueprints/Pawns/ShooterCharacter_BP Object Reference"))
  (bind _output_get (set `self.LastGrabber` `Last Grabber`))
  (set `self.Instigator` _output_get))

(fn `UserConstructionScript`)