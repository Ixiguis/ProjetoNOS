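; Jumppad is an environment actor that launches shooter characters and projectiles overlapping its static mesh along an arrow's forward direction at a configurable launch velocity.
; Characters use LaunchCharacter with optional XY and Z override, while projectiles with non-zero initial speed get their movement velocity replaced.
; The construction script pitches the arrow by Angle and passes the resulting launch vector to the particle system, so the effect follows the launch settings.
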(event `self.StaticMesh.OnComponentBeginOverlap`
  (params (OverlappedComponent :type "PrimitiveComponent Object Reference") (OtherActor :type "Actor Object Reference") (OtherComp :type "PrimitiveComponent Object Reference") (OtherBodyIndex :type Integer) (bFromSweep :type Boolean) (SweepResult :type "HitResult Structure (by ref)"))
  (bind _returnvalue (* (`SceneComponent.GetForwardVector` (`self.Arrow`)) (`self.LaunchVelocity`)))
  (bind _asshooter_character_bp (cast `/Game/Blueprints/Pawns/ShooterCharacter_BP` OtherActor)
    (:`then`
      (`Character.LaunchCharacter` _asshooter_character_bp _returnvalue (`self.ReplaceXYVel`) (`self.ReplaceZVel`)))
    (:`CastFailed`
      (bind _asshooter_projectile (cast `ShooterProjectile` OtherActor))
      (bind _movementcomp (`ShooterProjectile.MovementComp` _asshooter_projectile))
      (if (!= (`ProjectileMovementComponent.InitialSpeed` _movementcomp) 0.0)
        (set `MovementComponent.Velocity` _returnvalue _movementcomp)))))

(fn `UserConstructionScript`
  (`SceneComponent.K2_SetRelativeRotation` (`self.Arrow`) (`KismetMathLibrary.MakeRotator` 0.0 (`self.Angle`)) false false)
  (`ParticleSystemComponent.SetVectorParameter` (`self.ParticleSystem`) "LaunchVelocity" (* (`SceneComponent.GetForwardVector` (`self.Arrow`)) (`self.LaunchVelocity`))))