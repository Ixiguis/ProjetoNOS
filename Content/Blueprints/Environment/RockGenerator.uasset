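; RockGenerator is an environment Blueprint that produces a randomized rock variant from a single static mesh component.
; Its construction script picks a random mesh from the Meshes array and gives it a random rotation, including roll.
; Each scale axis varies independently around 1.0 within ScaleAdjustmentRange, allowing non-uniform shapes.
; The randomness is unseeded, so the look changes whenever the construction script reruns.
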(fn `UserConstructionScript`
  (bind _scaleadjustmentrange (`self.ScaleAdjustmentRange`))
  (bind _meshes (`self.Meshes`))
  (bind _returnvalue (- 1.0 _scaleadjustmentrange))
  (bind _returnvalue_2 (+ 1.0 _scaleadjustmentrange))
  (`SceneComponent.SetRelativeScale3D` (`self.StaticMesh1`) (`KismetMathLibrary.MakeVector` (`KismetMathLibrary.RandomFloatInRange` _returnvalue _returnvalue_2) (`KismetMathLibrary.RandomFloatInRange` _returnvalue _returnvalue_2) (`KismetMathLibrary.RandomFloatInRange` _returnvalue _returnvalue_2)))
  (`SceneComponent.K2_SetRelativeRotation` (`self.StaticMesh1`) (`KismetMathLibrary.RandomRotator` true) false false)
  (`StaticMeshComponent.SetStaticMesh` (`self.StaticMesh1`) (`KismetArrayLibrary.Array_Get` _meshes (`KismetMathLibrary.RandomIntegerInRange` 0 (- (`KismetArrayLibrary.Array_Length` _meshes) 1)))))