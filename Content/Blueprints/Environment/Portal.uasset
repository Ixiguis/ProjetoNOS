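; Portal actor that teleports whatever overlaps its collision shape to a Destination.
; Destination's location is relative to the portal's location and rotation, while its rotation applies as world-space facing.
; Characters trigger it only through their capsule and get their control rotation snapped to the exit facing.
; Physics linear velocity is zeroed on the overlapping component, while movement components keep their speed, redirected along the exit's forward vector.
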(event `self.CollisionShape.OnComponentBeginOverlap`
  (params (OverlappedComponent :type "PrimitiveComponent Object Reference") (OtherActor :type "Actor Object Reference") (OtherComp :type "PrimitiveComponent Object Reference") (OtherBodyIndex :type Integer) (bFromSweep :type Boolean) (SweepResult :type "HitResult Structure (by ref)"))
  (bind _rotation (.rotation (`self.Destination`)))
  (bind _ascharacter (cast `Character` OtherActor)
    (:`then`
      (if (== (`Character.CapsuleComponent` _ascharacter) OtherComp)
        (`Controller.SetControlRotation` (`Pawn.GetController` _ascharacter) _rotation)
        (`PrimitiveComponent.SetPhysicsLinearVelocity` OtherComp (0.0 0.0 0.0) false "None" :!label _label)
        (`self.K2_TeleportTo` OtherActor (+ (`KismetMathLibrary.GreaterGreater_VectorRotator` (.location (`self.Destination`)) (`self.K2_GetActorRotation`)) (`self.K2_GetActorLocation`)) _rotation)
        (for _array_element (`self.K2_GetComponentsByClass` OtherActor "/Script/Engine.MovementComponent")
          (bind _asmovement_component (cast `MovementComponent` _array_element))
          (set `MovementComponent.Velocity` (* (`KismetMathLibrary.Conv_RotatorToVector` _rotation) (`KismetMathLibrary.VSize` (`MovementComponent.Velocity` _asmovement_component))) _asmovement_component) ; set all movement components (if any) velocity to their current velocity, pointing to wherever the Destination's rotation is pointing
        )))
    (:`CastFailed`
      (goto _label))))

(fn `UserConstructionScript`)