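; Mjolnir lightning weapon with primary fire and a charged secondary discharge.
; ReleaseCharge scales damage by charge time, then chains from the trace impact to the nearest visible unhit character within range, reducing damage if the first hit misses a character.
; Fire and charge state drive the arm animation and, through UpdateMaterials on Tick, cupola, contact and valve particles.
; Reaching max charge sets BlownUp, whose OnRep explodes the weapon, heavily damaging and ragdolling its owner.
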(event `self.SimulateWeaponFireEvent`
  (params (FireMode :type Byte) (InMuzzlePSC :type "ParticleSystemComponent Object Reference"))
  (if (== FireMode 0)
    (set `self.FiringPrimary` true)
    (`self.SetArmAnim` true)))

(event `self.StopSimulatingWeaponFireEvent`
  (params (FireMode :type Byte))
  (if (== FireMode 0)
    (set `self.FiringPrimary` false)
    (`self.SetArmAnim` false)))

(event `self.WeaponStartChargeEvent`
  (params (FireMode :type Byte))
  (`AudioComponent.Play` (`self.ChargeAudio`) 0.0)
  (`KismetSystemLibrary.Delay` (`self.MinChargeTime`))
  (if (`self.IsCharging`)
    (`self.SetArmAnim` true)))

(event `self.WeaponStopChargeEvent`
  (params (FireMode :type Byte) (TotalChargingTime :type "Float (single-precision)"))
  (if (> TotalChargingTime (`self.MinChargeTime`))
    (`self.ReleaseCharge`))
  (`AudioComponent.Stop` (`self.ChargeAudio`))
  (`KismetSystemLibrary.Delay` 0.6)
  (`self.SetArmAnim` false))

(event `self.WeaponMaxChargeReachedEvent`
  (params (FireMode :type Byte) (TotalChargingTime :type "Float (single-precision)"))
  (set `self.BlownUp` true))

(event `self.ReceiveTick`
  (params (DeltaSeconds :type "Float (single-precision)"))
  (`parent.ReceiveTick` DeltaSeconds)
  (if (`self.IsEquipped`)
    (`self.UpdateMaterials` DeltaSeconds)))

(event `self.WeaponBeingEquippedEvent`
  ;[1 1 1] Spawn particles
  (bind _returnvalue (`GameplayStatics.SpawnEmitterAttached` "/Game/Weapons/Mjolnir/P_Mjolnir_Contact.P_Mjolnir_Contact" (`self.GetWeaponMesh`) "Cupola_contact" (0.0 0.0 0.0) (struct) (1.0 1.0 1.0) "KeepRelativeOffset" false))
  (bind _output_get (set `self.ContactPSC` _returnvalue))
  (`ParticleSystemComponent.SetVectorParameter` _output_get "Intensity" (0.0 0.0 0.0))
  (bind _returnvalue_2 (`GameplayStatics.SpawnEmitterAttached` "/Game/Weapons/Mjolnir/P_Mjolnir_CupolaLighting.P_Mjolnir_CupolaLighting" (`self.GetWeaponMesh`) "Cupola_center" (0.0 0.0 0.0) (struct) (1.0 1.0 1.0) "KeepRelativeOffset" false))
  (bind _output_get_2 (set `self.CupolaLightingPSC` _returnvalue_2))
  (`ParticleSystemComponent.SetVectorParameter` _output_get_2 "Intensity" (0.0 0.0 0.0))
  ;;[1 0 0] Valves lighting
  (bind _returnvalue_3 (`GameplayStatics.SpawnEmitterAttached` "/Game/Weapons/Mjolnir/P_Mjolnir_ValveLighting.P_Mjolnir_ValveLighting" (`self.GetWeaponMesh`) "Tube_Lighting_1" (0.0 0.0 0.0) (struct) (1.0 1.0 1.0) "KeepRelativeOffset" false))
  (bind _output_get_3 (set `self.ValvePSC_1` _returnvalue_3))
  (`ParticleSystemComponent.SetVectorParameter` _output_get_3 "Intensity" (0.0 0.0 0.0))
  (bind _returnvalue_4 (`GameplayStatics.SpawnEmitterAttached` "/Game/Weapons/Mjolnir/P_Mjolnir_ValveLighting.P_Mjolnir_ValveLighting" (`self.GetWeaponMesh`) "Tube_Lighting_2" (0.0 0.0 0.0) (struct) (1.0 1.0 1.0) "KeepRelativeOffset" false))
  (bind _output_get_4 (set `self.ValvePSC_2` _returnvalue_4))
  (`ParticleSystemComponent.SetVectorParameter` _output_get_4 "Intensity" (0.0 0.0 0.0))
  (bind _returnvalue_5 (`GameplayStatics.SpawnEmitterAttached` "/Game/Weapons/Mjolnir/P_Mjolnir_ValveLighting.P_Mjolnir_ValveLighting" (`self.GetWeaponMesh`) "Tube_Lighting_3" (0.0 0.0 0.0) (struct) (1.0 1.0 1.0) "KeepRelativeOffset" false))
  (bind _output_get_5 (set `self.ValvePSC_3` _returnvalue_5))
  (`ParticleSystemComponent.SetVectorParameter` _output_get_5 "Intensity" (0.0 0.0 0.0))
  (bind _returnvalue_6 (`GameplayStatics.SpawnEmitterAttached` "/Game/Weapons/Mjolnir/P_Mjolnir_ValveLighting.P_Mjolnir_ValveLighting" (`self.GetWeaponMesh`) "Tube_Lighting_4" (0.0 0.0 0.0) (struct) (1.0 1.0 1.0) "KeepRelativeOffset" false))
  (bind _output_get_6 (set `self.ValvePSC_4` _returnvalue_6))
  (`ParticleSystemComponent.SetVectorParameter` _output_get_6 "Intensity" (0.0 0.0 0.0)))

(event `self.WeaponUnequippedEvent`
  ;[1 1 1] Spawn particles
  (`ActorComponent.K2_DestroyComponent` (`self.ContactPSC`))
  (`ActorComponent.K2_DestroyComponent` (`self.CupolaLightingPSC`)))

(fn `GetClosestCharacterForChainLightning`
  (params (Characters :type "Array of Actor Object Reference (by ref)"))
  (returns (Character :type "ShooterCharacter Object Reference") (Found :type Boolean))
  (bind _closestcharacter (`self.ClosestCharacter`))
  (`|ExecutionSequence`
    (:`then_0`
      ;[1 1 1] 1. Find characters that are in line of sight of impact point
      (`KismetArrayLibrary.Array_Clear` (`self.UnblockedCharacters`))
      (set `self.I` 0)
      (while (< (`self.I`) (`KismetArrayLibrary.Array_Length` Characters))
        (bind _asshooter_character (cast `ShooterCharacter` (`|GetArrayItem` Characters (`self.I`))))
        (bind (_outhit _returnvalue) (`KismetSystemLibrary.LineTraceSingleForObjects` (`self.LightningTestFrom`) (`self.K2_GetActorLocation` _asshooter_character) (`self.World`) false (`self.CharactersHitByLighting`)))
        (if (not _returnvalue)
          (`KismetArrayLibrary.Array_Add` (`self.UnblockedCharacters`) _asshooter_character))
        (set `self.I` (+ (`self.I`) 1))))
    (:`then_1`
      ;[1 1 1] 2. Find closest character to source
      (set `self.ClosestCharacter` null)
      (set `self.ClosestDist` 10000.0)
      (for _array_element (`self.UnblockedCharacters`)
        (bind _asshooter_character_2 (cast `ShooterCharacter` _array_element))
        (bind _returnvalue_2 (`KismetMathLibrary.VSize` (- (`self.K2_GetActorLocation` _array_element) (`self.LightningTestFrom`))))
        (if (< _returnvalue_2 (`self.ClosestDist`))
          (set `self.ClosestDist` _returnvalue_2)
          (set `self.ClosestCharacter` _asshooter_character_2))))
    (:`then_2`
      ;[1 1 1] 3. Return closest character
      (return _closestcharacter (!= _closestcharacter null)))))

(fn `OnRep_BlownUp`
  (bind _returnvalue (`self.GetPawnOwner`))
  (bind _returnvalue_2 (`self.GetPawnOwnerController`))
  (bind _ownermesh (`self.OwnerMesh`))
  (set `self.OwnerMesh` (`ShooterCharacter.GetPawnMesh3P` (`self.GetPawnOwner`)))
  (set `self.WeaponWorldLocation` (`SceneComponent.K2_GetComponentLocation` (`self.GetWeaponMesh3P`)))
  (`GameplayStatics.SpawnEmitterAtLocation` "/Game/Effects/Particles/P_Fireball_Explosion.P_Fireball_Explosion" (`self.WeaponWorldLocation`))
  (`GameplayStatics.PlaySoundAtLocation` "/Game/Sounds/Weapons/GrenadeLauncher/GrenadeLauncher_Explosion_Cue.GrenadeLauncher_Explosion_Cue" (`self.WeaponWorldLocation`) (struct) 1.0 1.0 0.0 null null null)
  (`GameplayStatics.ApplyRadialDamage` 300.0 (`self.WeaponWorldLocation`) 512.0 "/Game/Blueprints/DamageTypes/DmgType_Explosion.DmgType_Explosion_C" (`|MakeArray` _returnvalue :!type "Actor Object Reference") self _returnvalue_2)
  (`GameplayStatics.ApplyDamage` _returnvalue 10000.0 _returnvalue_2 self "/Game/Blueprints/DamageTypes/DmgType_Explosion.DmgType_Explosion_C")
  ;[1 1 1] Activate ragdoll right now! (so that AddImpulse works on clients; their pawn isn't dead yet until replication)
  (`PrimitiveComponent.SetSimulatePhysics` _ownermesh true)
  (`PrimitiveComponent.SetCollisionEnabled` _ownermesh "QueryAndPhysics")
  (`PrimitiveComponent.AddImpulse` _ownermesh (0.0 0.0 10000.0) "None" true))

(fn `ReleaseCharge`
  (bind _returnvalue (`self.WeaponTrace` (0.0 0.0 0.0) (0.0 0.0 0.0) null))
  (bind _intensity (`self.CalculateIntensity`))
  (bind (_bblockinghit _binitialoverlap _time _distance _location _impactpoint _normal _impactnormal _physmat _hitactor) (`GameplayStatics.BreakHitResult` _returnvalue))
  (`GameplayStatics.PlaySoundAtLocation` "/Game/Sounds/Weapons/Mjolnir/MJOLNIR_SEC_FIRE_Cue.MJOLNIR_SEC_FIRE_Cue" (`self.K2_GetActorLocation` (`self.GetPawnOwner`)) (struct) 1.0 1.0 0.0 null null null)
  (bind _returnvalue_2 (`GameplayStatics.SpawnEmitterAttached` "/Game/Weapons/Mjolnir/P_Mjolnir_CupolaLighting_Discharge.P_Mjolnir_CupolaLighting_Discharge" (`self.GetWeaponMesh`) "Cupola_center"))
  (`ParticleSystemComponent.SetFloatParameter` _returnvalue_2 "Intensity" (`self.GetChargingPercent`))
  ;[1 1 1] First hit
  (set `self.DamageToDeal` (* (`self.AltFireBaseDamage`) (`self.GetChargingTime`)))
  (`KismetArrayLibrary.Array_Clear` (`self.CharactersHitByLighting`))
  (bind _returnvalue_3 (`GameplayStatics.SpawnEmitterAttached` "/Game/Weapons/Mjolnir/P_Mjolnir_Secondary.P_Mjolnir_Secondary" (`self.GetWeaponMesh`) (`|GetArrayItem` (`self.MuzzleAttachPoint`))))
  (`ParticleSystemComponent.SetVectorParameter` _returnvalue_3 "Intensity" _intensity)
  (`ParticleSystemComponent.SetFloatParameter` _returnvalue_3 "Intensity" (.x _intensity))
  (`self.SpawnImpactEffects` _returnvalue)
  (`ParticleSystemComponent.SetVectorParameter` _returnvalue_3 (`self.TrailTargetParam`) _impactpoint)
  (set `self.LightningTestFrom` (+ _impactpoint (* _impactnormal (10.0 10.0 10.0))))
  (`GameplayStatics.ApplyDamage` _hitactor (`self.DamageToDeal`) (`self.GetPawnOwnerController`) self "/Game/Blueprints/DamageTypes/DmgType_Instant.DmgType_Instant_C")
  (bind _asshooter_character (cast `ShooterCharacter` _hitactor)
    (:`then`
      (`KismetArrayLibrary.Array_Add` (`self.CharactersHitByLighting`) _asshooter_character))
    (:`CastFailed`
      (set `self.DamageToDeal` (* (`self.MissDamageMultiplier`) (`self.DamageToDeal`)))))
  ;[1 1 1] Secondary hits
  (bind _outactors (`KismetSystemLibrary.SphereOverlapActors` (`self.LightningTestFrom`) (`self.JumpMaxDistance`) (`self.Pawns`) "/Script/ShooterGame.ShooterCharacter" (`self.CharactersHitByLighting`) :!label _label))
  (bind (_character _found) (`self.GetClosestCharacterForChainLightning` _outactors))
  (if _found
    (`GameplayStatics.ApplyDamage` _character (`self.DamageToDeal`) (`self.GetPawnOwnerController`) self "/Game/Blueprints/DamageTypes/DmgType_Instant.DmgType_Instant_C")
    (`KismetArrayLibrary.Array_Add` (`self.CharactersHitByLighting`) _character)
    (bind _returnvalue_4 (`GameplayStatics.SpawnEmitterAtLocation` "/Game/Weapons/Mjolnir/P_Mjolnir_Secondary.P_Mjolnir_Secondary" (`self.LightningTestFrom`)))
    (bind _returnvalue_5 (`SceneComponent.GetSocketLocation` (`Character.Mesh` _character) "Heart"))
    (`ParticleSystemComponent.SetVectorParameter` _returnvalue_4 (`self.TrailTargetParam`) _returnvalue_5)
    (`ParticleSystemComponent.SetVectorParameter` _returnvalue_4 "Intensity" (`self.CalculateIntensity`))
    (set `self.LightningTestFrom` _returnvalue_5)
    (goto _label)
    (else
      (`self.UpdateMaterials` 0.0))))

(fn `UpdateMaterials`
  (params (DeltaTime :type "Float (double-precision)"))
  (bind _returnvalue (`self.GetWeaponMesh`))
  (bind _cupolatemperature (`self.CupolaTemperature`))
  (bind _contactpsc (`self.ContactPSC`))
  (bind _cupolalightingpsc (`self.CupolaLightingPSC`))
  (bind _valvepsc_1 (`self.ValvePSC_1`))
  ;[1 1 1] Determine cupola temperature
  (set `self.CupolaTemperature` (select `bool` (`self.FiringPrimary`) :`false` (- _cupolatemperature (* DeltaTime (`self.CupolaTemperatureDecreasePerSec`))) :`true` (+ (* DeltaTime (`self.CupolaTemperatureIncreasePerSec`)) _cupolatemperature)))
  ;[1 1 1] Has ammo?
  (if (<= (`self.GetCurrentAmmo`) 0)
    (`ParticleSystemComponent.SetVectorParameter` (`self.CupolaLightingPSC`) "Intensity" (0.0 0.0 0.0))
    (else
      ;[1 1 1] Define parameters for the ray that goes from cupola to arm when firing primary
      (`ParticleSystemComponent.SetVectorParameter` _contactpsc "Intensity" (select `bool` (`self.FiringPrimary`) :`false` (`KismetMathLibrary.MakeVector` 0.0) :`true` (`KismetMathLibrary.MakeVector` 1.0 1.0 1.0)))
      (`/Engine/EditorBlueprintResources/StandardMacros.IsValid` _returnvalue
        (:`Is Valid`
          (`ParticleSystemComponent.SetVectorParameter` _contactpsc "Target" (`SceneComponent.GetSocketLocation` _returnvalue "Arm_sphere"))
          ;[1 1 1] Cupola's lighting intensity
          (if (`self.IsCharging`)
            (`ParticleSystemComponent.SetVectorParameter` _cupolalightingpsc "Intensity" (`|EaseFunction` "ExpoOut" (* (`self.GetChargingPercent`) 2.0) (`self.CupolaLightingIdle`)))
            ;[1 1 1] Valves lighting intensity
            (`ParticleSystemComponent.SetVectorParameter` _valvepsc_1 "Intensity" (`|EaseFunction` "ExpoIn" (`self.GetChargingPercent`) (0.0 0.0 0.0) (1.0 1.0 1.0)))
            (`ParticleSystemComponent.SetVectorParameter` (`self.ValvePSC_2`) "Intensity" (`|EaseFunction` "ExpoIn" (`self.GetChargingPercent`) (0.0 0.0 0.0) (1.0 1.0 1.0)))
            (`ParticleSystemComponent.SetVectorParameter` (`self.ValvePSC_3`) "Intensity" (`|EaseFunction` "ExpoIn" (`self.GetChargingPercent`) (0.0 0.0 0.0) (1.0 1.0 1.0)))
            (`ParticleSystemComponent.SetVectorParameter` (`self.ValvePSC_4`) "Intensity" (`|EaseFunction` "ExpoIn" (`self.GetChargingPercent`) (0.0 0.0 0.0) (1.0 1.0 1.0)))
            (else
              (`ParticleSystemComponent.SetVectorParameter` _cupolalightingpsc "Intensity" (select `bool` (`self.FiringPrimary`) :`false` (`self.CupolaLightingIdle`) :`true` (`KismetMathLibrary.MakeVector` 1.0 1.0 1.0)))
              (`ParticleSystemComponent.SetVectorParameter` _valvepsc_1 "Intensity" (0.0 0.0 0.0))
              (`ParticleSystemComponent.SetVectorParameter` (`self.ValvePSC_2`) "Intensity" (0.0 0.0 0.0))
              (`ParticleSystemComponent.SetVectorParameter` (`self.ValvePSC_3`) "Intensity" (0.0 0.0 0.0))
              (`ParticleSystemComponent.SetVectorParameter` (`self.ValvePSC_4`) "Intensity" (0.0 0.0 0.0)))))))))

(fn `UserConstructionScript`
  (`parent.UserConstructionScript`))