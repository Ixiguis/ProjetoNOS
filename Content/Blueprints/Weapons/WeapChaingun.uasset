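; Chaingun weapon whose barrel spin rises while firing, with alt-fire either braking or boosting it depending on AltFireBoosts.
; Each tick, spin rate sets fire rate, dispersion and animation speed, doubling shots per tick to cap firing frequency.
; On the server, high spin pushes the owner backward and a looping timer damages them while firing.
; Spin also drives engine audio and accumulated muzzle and brake heat, shown through particles and material glow.
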(event `self.ReceiveDestroyed`
  (`ActorComponent.K2_DestroyComponent` (`self.SmokePSC`))
  (`ActorComponent.K2_DestroyComponent` (`self.FirePSC`))
  (`ActorComponent.K2_DestroyComponent` (`self.BrakePSC`))
  (`AudioComponent.FadeOut` (`self.EngineSoundComponent`) 0.5 0.0 "Linear"))

(event `self.ReceiveBeginPlay`
  (bind _returnvalue (`GameplayStatics.SpawnEmitterAtLocation` "/Game/Weapons/Chaingun/P_FiringSmoke.P_FiringSmoke"))
  (set `self.SmokePSC` _returnvalue)
  (bind _returnvalue_2 (`GameplayStatics.SpawnEmitterAtLocation` "/Game/Weapons/Chaingun/P_CHaingunFire.P_CHaingunFire"))
  (set `self.FirePSC` _returnvalue_2)
  (bind _returnvalue_3 (`GameplayStatics.SpawnEmitterAtLocation` "/Game/Weapons/Chaingun/P_Brake.P_Brake"))
  (set `self.BrakePSC` _returnvalue_3)
  (`self.UpdateEffects` 0.0))

(event `self.WeaponEquippedEvent`
  (`AudioComponent.FadeIn` (`self.EngineSoundComponent`) 0.5 1.0 0.0 "Linear")
  (`AudioComponent.FadeIn` (`self.BrakeAudioComponent`) 0.2 1.0 0.0 "Linear")
  (set `self.IsBraking` false)
  (`self.UpdateEffects` 0.0)
  (`/Engine/EditorBlueprintResources/ActorMacros.Switch Has Authority`
    (:`Authority`
      (`KismetSystemLibrary.K2_SetTimer` null "DamageOwner" 0.5 true))))

(event `self.WeaponUnequippedEvent`
  (`AudioComponent.FadeOut` (`self.EngineSoundComponent`) 0.5 0.0 "Linear")
  (`AudioComponent.FadeOut` (`self.BrakeAudioComponent`) 0.2 0.0 "Linear")
  (`self.UpdateEffects` 0.0)
  (`/Engine/EditorBlueprintResources/ActorMacros.Switch Has Authority`
    (:`Authority`
      (`KismetSystemLibrary.K2_ClearTimer` null "DamageOwner"))))

(event `self.UserStartedFiringEvent`
  (params (FireMode :type Byte))
  (if (and (== FireMode 0) (`self.HasEnoughAmmo`))
    (set `self.IsFiring` true)))

(event `self.UserStoppedFiringEvent`
  (params (FireMode :type Byte))
  (if (== FireMode 0)
    (set `self.IsFiring` false)))

(event `self.StartCustomFire`
  (params (FireMode :type Byte))
  (if (`self.AltFireBoosts`)
    (set `self.IsBoosting` true)
    (else
      (set `self.WantsToBrake` true))))

(event `self.StopCustomFire`
  (params (FireMode :type Byte))
  (if (`self.AltFireBoosts`)
    (set `self.IsBoosting` false)
    (else
      (set `self.WantsToBrake` false))))

(event `self.ReceiveTick`
  (params (DeltaSeconds :type "Float (single-precision)"))
  (`self.UpdateSpinRate` DeltaSeconds)
  (`self.UpdateEffects` DeltaSeconds)
  (`/Engine/EditorBlueprintResources/ActorMacros.Switch Has Authority`
    (:`Authority`
      (`self.PushOwner` DeltaSeconds))))

(fn `DamageOwner`
  (bind _returnvalue (`self.GetPawnOwner`))
  (bind _returnvalue_2 (`Pawn.GetController` _returnvalue))
  (bind _x (.x (`self.SpinSpeedDamageOwner`)))
  (bind _z (.z (`self.SpinSpeedDamageOwner`)))
  (bind _returnvalue_3 (`KismetMathLibrary.FMin` (`KismetMathLibrary.Lerp` 0.0 _z (/ (`KismetMathLibrary.FMax` (- (`self.CurrentSpinRate`) _x)) (- (.y (`self.SpinSpeedDamageOwner`)) _x))) _z))
  (if (and (!= _returnvalue null) (> (`ShooterCharacter.Health` _returnvalue) 0.0) (`self.IsFiring`) (> _returnvalue_3 0.0) (!= _returnvalue_2 null))
    (`GameplayStatics.ApplyDamage` _returnvalue _returnvalue_3 _returnvalue_2 self)))

(fn `OnRep_AltFireBoosts`
  (if (`self.AltFireBoosts`)
    (set `self.InitialSpinRate` (`self.Boost_InitialSpinRate`))
    (set `self.AccelerationFiring` (`self.Boost_BoostAcceleration`))
    (set `self.Deacceleration` (`self.Boost_Deacceleration`))
    (set `self.CurrentSpinRate` (`self.InitialSpinRate`))))

(fn `OnRep_IsBraking`
  (bind _brakeaudiocomponent (`self.BrakeAudioComponent`))
  (if (`self.IsBraking`)
    (`AudioComponent.SetVolumeMultiplier` _brakeaudiocomponent 1.0)
    (else
      (`AudioComponent.SetVolumeMultiplier` _brakeaudiocomponent 0.0))))

(fn `UpdateEffects`
  (params (DeltaTime :type "Float (double-precision)"))
  (bind _currentspinrate (`self.CurrentSpinRate`))
  (bind _smokepsc (`self.SmokePSC`))
  (bind _returnvalue (`KismetMathLibrary.Lerp` (- _currentspinrate 70.0) _currentspinrate (`KismetMathLibrary.Conv_BoolToDouble` (`self.AltFireBoosts`))))
  (if (or (`self.IsEquipped`) (== DeltaTime 0.0) (> (`self.WeaponHeat`) 0.0))
    (if (`self.IsEquipped`)
      (if (`self.IsFiring`)
        (set `self.WeaponHeat` (+ (`self.WeaponHeat`) (* (* (`self.ShotsPerSec`) 0.5) DeltaTime))))
      (set `self.WeaponHeat` (`KismetMathLibrary.FMax` (- (`self.WeaponHeat`) (* DeltaTime (/ (`self.WeaponHeat`) 8.0)))))
      (`ParticleSystemComponent.SetFloatParameter` _smokepsc "SpawnRate" (`self.WeaponHeat`))
      (`ParticleSystemComponent.SetFloatParameter` (`self.FirePSC`) "SpawnRate" (`self.WeaponHeat`))
      (`SceneComponent.K2_SetWorldLocation` _smokepsc (`SceneComponent.GetSocketLocation` (`self.GetWeaponMesh`) "ExhaustSocket") false false)
      (`SceneComponent.K2_SetWorldLocation` (`self.FirePSC`) (`SceneComponent.GetSocketLocation` (`self.GetWeaponMesh`) "ExhaustSocket") false false)
      (`MaterialInstanceDynamic.SetScalarParameterValue` (`self.Material1P`) "MuzzleHeat" (`KismetMathLibrary.FClamp` (`KismetMathLibrary.MapRangeUnclamped` (`self.WeaponHeat`) 150.0 700.0 300.0 4500.0) 0.0 4500.0))
      (`MaterialInstanceDynamic.SetScalarParameterValue` (`self.Material3P`) "MuzzleHeat" (`KismetMathLibrary.FClamp` (`KismetMathLibrary.MapRangeUnclamped` (`self.WeaponHeat`) 150.0 700.0 300.0 4500.0) 0.0 4500.0))
      (else
        (`ParticleSystemComponent.SetFloatParameter` (`self.SmokePSC`) "SpawnRate" 0.0)
        (`ParticleSystemComponent.SetFloatParameter` (`self.FirePSC`) "SpawnRate" 0.0)))
    (`AudioComponent.SetPitchMultiplier` (`self.EngineSoundComponent`) (+ (/ _returnvalue 600.0) 0.35))
    (`AudioComponent.SetVolumeMultiplier` (`self.EngineSoundComponent`) (`KismetMathLibrary.FClamp` (/ _returnvalue 100.0) 0.3))
    (`SceneComponent.K2_SetWorldLocation` (`self.BrakePSC`) (`SceneComponent.GetSocketLocation` (`self.GetWeaponMesh`) "BrakeParticlesSocket") false false)
    (if (`self.IsBraking`)
      (`ParticleSystemComponent.SetFloatParameter` (`self.BrakePSC`) "SpawnRate" (`self.ShotsPerSec`))
      (set `self.BrakeHeat` (+ (`self.BrakeHeat`) (* (* (`self.ShotsPerSec`) 6.0) DeltaTime)))
      (else
        (`ParticleSystemComponent.SetFloatParameter` (`self.BrakePSC`) "SpawnRate" 0.0)))
    (set `self.BrakeHeat` (`KismetMathLibrary.FMax` (- (`self.BrakeHeat`) (* DeltaTime (/ (`self.BrakeHeat`) 1.5)))))
    (`MaterialInstanceDynamic.SetScalarParameterValue` (`self.Material1P`) "BrakeHeat" (`KismetMathLibrary.FClamp` (`KismetMathLibrary.MapRangeUnclamped` (`self.BrakeHeat`) 150.0 700.0 300.0 4500.0) 0.0 4500.0))
    (`MaterialInstanceDynamic.SetScalarParameterValue` (`self.Material3P`) "BrakeHeat" (`KismetMathLibrary.FClamp` (`KismetMathLibrary.MapRangeUnclamped` (`self.BrakeHeat`) 150.0 700.0 300.0 4500.0) 0.0 4500.0))))

(fn `UpdateSpinRate`
  (params (DeltaTime :type "Float (double-precision)"))
  (bind _isbraking (`self.IsBraking`))
  (if (`self.IsBraking`)
    ;[1 1 1] Apply brake
    (set `self.CurrentSpinRate` (- (`self.CurrentSpinRate`) (* (`self.DeaccelerationBraking`) DeltaTime))))
  ;[1 1 1] Accelerate / Deaccelerate
  (if (or (and (`self.IsFiring`) (not (`self.AltFireBoosts`))) (and (`self.AltFireBoosts`) (`self.IsBoosting`) (`self.IsFiring`) (`self.HasEnoughAmmo`)))
    (set `self.CurrentSpinRate` (+ (`self.CurrentSpinRate`) (* (`self.AccelerationFiring`) DeltaTime)))
    (else
      (set `self.CurrentSpinRate` (- (`self.CurrentSpinRate`) (* (`self.Deacceleration`) DeltaTime)))))
  ;[1 1 1] Discover the current fire rate
  (if (< (`self.CurrentSpinRate`) (`self.InitialSpinRate`))
    (set `self.CurrentSpinRate` (`self.InitialSpinRate`)))
  (set `self.ShotsPerSec` (* (`self.CurrentSpinRate`) 0.25))
  (set `self.TimeTweenShots` (/ 1.0 (`self.ShotsPerSec`)))
  ;[1 1 1] Prevent TimeBetweenShots from going too low (optimization)
  (`self.SetShotsPerTick` 0 1)
  (while (< (`self.TimeTweenShots`) (`self.MinTimeBetweenShots`))
    (`self.SetShotsPerTick` 0 (* (`self.GetShotsPerTick` 0) 2))
    (set `self.TimeTweenShots` (* (`self.TimeTweenShots`) 2.0)))
  ;[1 1 1] [Server] set actual fire rate and firing spread
  (`self.SetFireRate` 0 (`self.TimeTweenShots`))
  (`self.SetCurrentFiringDispersion` (+ (* (- (`self.CurrentSpinRate`) (`self.InitialSpinRate`)) (`self.DispersionFactor`)) (`self.GetBaseFiringDispersion`)))
  ;[1 1 1] Set SpinRate for the Anim BP
  (bind _aschaingun_anim_bp (cast `/Game/Weapons/Chaingun/ChaingunAnimBP` (`SkeletalMeshComponent.GetAnimInstance` (`self.Mesh1P`))))
  (set `/Game/Weapons/Chaingun/ChaingunAnimBP.SpinRate` (`self.CurrentSpinRate`) _aschaingun_anim_bp)
  (bind _aschaingun_anim_bp_2 (cast `/Game/Weapons/Chaingun/ChaingunAnimBP` (`SkeletalMeshComponent.GetAnimInstance` (`self.Mesh3P`))))
  (set `/Game/Weapons/Chaingun/ChaingunAnimBP.SpinRate` (`self.CurrentSpinRate`) _aschaingun_anim_bp_2)
  ;[1 1 1] Set IsBraking (Only modify if it changed to save bandwidth)
  (if (and (`self.WantsToBrake`) (> (`self.CurrentSpinRate`) (`self.InitialSpinRate`)))
    (if (not _isbraking)
      (set `self.IsBraking` true))
    (elif _isbraking
      (set `self.IsBraking` false))))

(fn `UserConstructionScript`
  (`parent.UserConstructionScript`)
  (set `self.CurrentSpinRate` (`self.InitialSpinRate`)))