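; Melee sword weapon with a chargeable slash, blocking, and health recovery for the wielder based on damage dealt.
; Charge events play montages; an anim notify calls Slash, which on the server damages each unique actor overlapping MeleeReach, scaled by capped charge time.
; Targets blocking with a sword only trigger a clash sound.
; While equipped and blocking, MeleeReach overlaps reverse deflectable projectiles and make the blocker their instigator.
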(event `self.WeaponStartChargeEvent`
  (params (FireMode :type Byte))
  (bind _returnvalue (`self.GetPawnOwner`))
  ;[1 1 1] Play animations and sounds. Slash() is called from the anim notify.
  (`Character.PlayAnimMontage` _returnvalue "/Game/Characters/Animations/FPP_Animations/FP_SwordCharge.FP_SwordCharge" 1.5 "None")
  (`Character.PlayAnimMontage` _returnvalue "/Game/Characters/HeroTPP/Sword_charge.Sword_charge" 1.5 "None"))

(event `self.WeaponStopChargeEvent`
  (params (FireMode :type Byte) (TotalChargingTime :type "Float (single-precision)"))
  (bind _returnvalue (`self.GetPawnOwner`))
  ;[1 1 1] Play animations and sounds. Slash() is called from the anim notify.
  (`Character.StopAnimMontage` _returnvalue "/Game/Characters/Animations/FPP_Animations/FP_SwordCharge.FP_SwordCharge")
  (`Character.StopAnimMontage` _returnvalue "/Game/Characters/HeroTPP/Sword_charge.Sword_charge")
  (`Character.PlayAnimMontage` _returnvalue "/Game/Characters/Animations/FPP_Animations/FP_SwordAttack2.FP_SwordAttack2" 1.0 "None")
  (`Character.PlayAnimMontage` _returnvalue "/Game/Characters/HeroTPP/SWORD_SLASH.SWORD_SLASH" 1.0 "None")
  (`GameplayStatics.SpawnSoundAttached` "/Game/Sounds/Weapons/Sword/SWORD_AIR_SLASH_Cue.SWORD_AIR_SLASH_Cue" (`self.GetWeaponMesh`) "None" (0.0 0.0 0.0) (struct) "KeepRelativeOffset" false 1.0 1.0 0.0 null null))

(event `self.WeaponEquippedEvent`
  ;[1 1 1] Start listening for overlap events on melee hit box
  (bind _asshooter_character_bp (cast `/Game/Blueprints/Pawns/ShooterCharacter_BP` (`self.GetPawnOwner`)))
  (add `PrimitiveComponent.OnComponentBeginOverlap` (`/Game/Blueprints/Pawns/ShooterCharacter_BP.MeleeReach` _asshooter_character_bp) (delegate `OnComponentBeginOverlap_Event`)))

(event `OnComponentBeginOverlap_Event`
  (params (OverlappedComponent :type "PrimitiveComponent Object Reference") (OtherActor :type "Actor Object Reference") (OtherComp :type "PrimitiveComponent Object Reference") (OtherBodyIndex :type Integer) (bFromSweep :type Boolean) (SweepResult :type "HitResult Structure (by ref)"))
  ;[1 1 1] Reflect incoming projectiles, if blocking
  (if (`self.IsBlocking`)
    (bind _asshooter_projectile (cast `ShooterProjectile` OtherActor))
    (bind _movementcomp (`ShooterProjectile.MovementComp` _asshooter_projectile))
    (bind _velocity (`MovementComponent.Velocity` _movementcomp))
    (if (and (`ShooterProjectile.CanBeDeflected` _asshooter_projectile) (> (`KismetMathLibrary.VSize` _velocity) 0.0))
      (set `MovementComponent.Velocity` (- (0.0 0.0 0.0) _velocity) _movementcomp)
      (`ShooterProjectile.SetInstigator` _asshooter_projectile (`self.GetPawnOwner`)) ; set projectile instigator to owner, so reflected missiles give credit to the blocker
      (`GameplayStatics.SpawnSoundAttached` "/Game/Sounds/Weapons/Sword/SWORD_SLASH_Cue.SWORD_SLASH_Cue" (`self.Mesh3P`) "None" (0.0 0.0 0.0) (struct) "KeepRelativeOffset" false 1.0 1.0 0.0 null null))))

(event `self.WeaponUnequippedEvent`
  ;[1 1 1] Stop listening for overlap events on melee hit box
  (bind _asshooter_character_bp (cast `/Game/Blueprints/Pawns/ShooterCharacter_BP` (`self.GetPawnOwner`)))
  (remove `PrimitiveComponent.OnComponentBeginOverlap` (`/Game/Blueprints/Pawns/ShooterCharacter_BP.MeleeReach` _asshooter_character_bp) (delegate `OnComponentBeginOverlap_Event`)))

(fn `RecoverHealth`
  (params (HitActor :type "Actor Object Reference") (DamageDealt :type "Float (double-precision)"))
  (bind _returnvalue (`self.GetPawnOwner`))
  (`/Engine/EditorBlueprintResources/ActorMacros.Switch Has Authority`
    (:`Authority`
      (bind _asshooter_character (cast `ShooterCharacter` HitActor))
      (if (> (`ShooterCharacter.Health` _asshooter_character) 0.0)
        (set `ShooterCharacter.Health` (`KismetMathLibrary.FMin` (+ (`ShooterCharacter.Health` _returnvalue) (* DamageDealt (`self.HealthRestoredFraction`))) (`ShooterCharacter.MaxBoostedHealth` _returnvalue)) _returnvalue)))))

(fn `Slash`
  (bind _variable (`|TemporaryVariable`))
  (bind _returnvalue (`KismetMathLibrary.Conv_IntToDouble` (+ (`self.GetInstantHitDamage` 0) (`KismetMathLibrary.Round` (* (`self.DamagePerSecCharging`) (`KismetMathLibrary.FClamp` (`self.GetChargingTime`) 0.0 2.0))))))
  (`/Engine/EditorBlueprintResources/ActorMacros.Switch Has Authority`
    (:`Authority`
      (bind _actorhit (`self.GetActorsHit`)
        (:`Loop`
          (bind _asshooter_character (cast `ShooterCharacter` _actorhit)
            (:`then`
              (bind _returnvalue_2 (`ShooterCharacter.GetWeapon` _asshooter_character))
              (if (!= _returnvalue_2 null)
                (bind _asweap_sword (cast `/Game/Blueprints/Weapons/WeapSword` _returnvalue_2)
                  (:`then`
                    (if (`/Game/Blueprints/Weapons/WeapSword.IsBlocking` _asweap_sword)
                      (`GameplayStatics.SpawnSoundAttached` "/Game/Sounds/Weapons/Sword/SWORD_SLASH_Cue.SWORD_SLASH_Cue" (`self.Mesh3P`) "None" (0.0 0.0 0.0) (struct) "KeepRelativeOffset" false 1.0 1.0 0.0 null null)
                      (else
                        (bind _asshooter_game_mode (cast `ShooterGameMode` (`GameplayStatics.GetGameMode`) :!label _label))
                        (`self.RecoverHealth` _actorhit (`ShooterGameMode.ModifyDamage` _asshooter_game_mode _returnvalue _actorhit (`self.GetPawnOwnerController`)))
                        (bind _asshooter_character_2 (cast `ShooterCharacter` _actorhit)
                          (:`then`
                            (`|AssignmentStatement` _variable (> (`ShooterCharacter.Health` _asshooter_character_2) 0.0)))
                          (:`CastFailed`
                            (`|AssignmentStatement` _variable)))
                        (`GameplayStatics.ApplyDamage` _actorhit _returnvalue (`self.GetPawnOwnerController`) self)
                        (`self.SlashEventDispatcher` _variable _returnvalue))))
                  (:`CastFailed`
                    (goto _label)))
                (else
                  (goto _label))))
            (:`CastFailed`
              (goto _label))))))))

(fn `UserConstructionScript`
  (`parent.UserConstructionScript`)
  (set `self.IsBlocking` false))