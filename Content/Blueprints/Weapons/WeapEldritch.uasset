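; WeapEldritch is a weapon Blueprint that tracks which fire mode is being held.
; StartCustomFire sets HoldingPrimary for mode 0 or HoldingSecondary for any other mode, clearing the opposite flag, and StopCustomFire clears both.
; HoldingPrimary has a RepNotify whose branch does nothing, and the construction script only calls its parent.
; No firing behavior or effects are implemented in these graphs.
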(event `self.StartCustomFire`
  (params (FireMode :type Byte))
  (if (== FireMode 0)
    (set `self.HoldingPrimary` true)
    (set `self.HoldingSecondary` false)
    (else
      (set `self.HoldingSecondary` true)
      (set `self.HoldingPrimary` false))))

(event `self.StopCustomFire`
  (params (FireMode :type Byte))
  (set `self.HoldingPrimary` false)
  (set `self.HoldingSecondary` false))

(fn `OnRep_HoldingPrimary`
  (if (`self.HoldingPrimary`)
    _))

(fn `UserConstructionScript`
  (`parent.UserConstructionScript`))