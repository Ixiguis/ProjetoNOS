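; Squid weapon that fires its primary mode as a spray with periodic pauses and regains ammo by eating character corpses.
; While equipped, a looping timer runs a locally controlled camera trace against physics bodies, plays eating and delayed belch sounds, and asks the server for ammo, which checks corpse distance.
; Pauses come from temporarily lengthening the time between shots after each spray interval or when firing stops.
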(event `self.WeaponEquippedEvent`
  (`KismetSystemLibrary.K2_SetTimer` null "CheckFood" 1.0 true))

(event `self.WeaponUnequippedEvent`
  (`KismetSystemLibrary.K2_ClearTimer` null "CheckFood"))

(event `ServerGiveSquidAmmo`
  (params (FoodCharacter :type "/Game/Blueprints/Pawns/ShooterCharacter_BP Object Reference"))
  (if (<= (`KismetMathLibrary.VSize` (- (`self.K2_GetActorLocation` FoodCharacter) (`self.K2_GetActorLocation` (`self.GetPawnOwner`)))) (`self.MaxCorpseDistance`))
    (`self.GiveAmmo` (`self.FeedAmmo`))))

(event `self.WeaponPreFireEvent`
  (params (FireMode :type Byte))
  (bind _spraypause (`self.SprayPause`))
  (if (and (== FireMode 0) (>= (- (`KismetSystemLibrary.GetGameTimeInSeconds`) (`self.LastPauseTime`)) (`self.SprayInterval`)))
    (`self.SetFireRate` 0 _spraypause :!label _label)
    (`KismetSystemLibrary.Delay` _spraypause)
    (`self.SetFireRate` 0 0.05)
    (set `self.LastPauseTime` (`KismetSystemLibrary.GetGameTimeInSeconds`))))

(event `self.UserStartedFiringEvent`
  (params (FireMode :type Byte))
  (if (== FireMode 0)
    (set `self.LastPauseTime` (`KismetSystemLibrary.GetGameTimeInSeconds`))))

(event `self.UserStoppedFiringEvent`
  (params (FireMode :type Byte))
  (if (== FireMode 0)
    (goto _label)))

(fn `Belch`
  (`GameplayStatics.SpawnSoundAttached` "/Game/Sounds/Weapons/Squid/SQUID_BELCH_Cue.SQUID_BELCH_Cue" (`self.GetWeaponMesh`) "None" (0.0 0.0 0.0) (struct) "KeepRelativeOffset" false 1.0 1.0 0.0 null null))

(fn `CheckFood`
  (bind _returnvalue (`self.GetPawnOwner`))
  (bind _returnvalue_2 (`self.GetPawnOwner`))
  (bind _tracestart (`self.TraceStart`))
  (if (`Pawn.IsLocallyControlled` (`self.GetPawnOwner`))
    (set `self.TraceStart` (`SceneComponent.GetSocketLocation` (`Character.Mesh` _returnvalue) "CameraLocation"))
    (bind (_outhit _returnvalue_3) (`KismetSystemLibrary.LineTraceSingleForObjects` _tracestart (+ _tracestart (* (`KismetMathLibrary.Conv_RotatorToVector` (`Pawn.GetControlRotation` _returnvalue)) (`self.FoodTraceDistance`))) (`self.ObjectsToTest`) true (`|MakeArray` _returnvalue :!type "Actor Object Reference")))
    (if _returnvalue_3
      (bind _asshooter_character_bp (cast `/Game/Blueprints/Pawns/ShooterCharacter_BP` (`.HitActor` (`GameplayStatics.BreakHitResult` _outhit))) ; No need to check pawn health, as the trace only tests PhysicsBody objects (not Pawns)
        (:`then`
          (`self.ServerGiveSquidAmmo` _asshooter_character_bp)
          (set `self.IsFeeding` true)
          (if (and (!= _returnvalue_2 null) (`Pawn.IsLocallyControlled` _returnvalue_2))
            (`GameplayStatics.SpawnSoundAttached` "/Game/Sounds/Weapons/Squid/SQUID_EAT_Cue.SQUID_EAT_Cue" (`self.Mesh1P`) "None" (0.0 0.0 0.0) (struct) "KeepRelativeOffset" false 1.0 1.0 0.0 null null)
            (`KismetSystemLibrary.K2_SetTimer` null "Belch" 5.0)))
        (:`CastFailed`
          (set `self.IsFeeding` false))))))

(fn `UserConstructionScript`
  (`parent.UserConstructionScript`))