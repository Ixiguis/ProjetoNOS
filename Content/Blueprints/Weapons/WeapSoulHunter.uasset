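; Soul Hunter shotgun that banks souls from its instant-hit kills, including any held by the victim's Soul Hunter, to speed up its wielder while equipped.
; Alt-fire spends them for multiplied damage and soul-scaled effects; those kills earn none, and idle souls decay on a looping timer.
; SoulsClaimed's OnRep updates speed and timeline-blended material glow.
; Daemon summoning is unfinished: the over-cap roll exists, but its follow-up is disconnected.
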(event `self.WeaponEquippedEvent`
  ;[1 1 1] Initialization
  (`self.SetCharacterSpeed` true))

(event `self.WeaponUnequippedEvent`
  ;[1 1 1] Initialization
  (`self.SetCharacterSpeed` false))

(event `self.KilledEvent`
  (params (KilledPawn :type "Pawn Object Reference") (KilledPlayer :type "Controller Object Reference") (KillerWeaponClass :type "ShooterWeapon Class Reference") (KillerDmgType :type "ShooterDamageType Class Reference"))
  (bind _soulsclaimed (`self.SoulsClaimed`))
  ;[1 1 1] Scored a kill: increase SoulsClaimed (Server)
  (if (and (== KillerWeaponClass "WeapSoulHunter_C") (== KillerDmgType "/Game/Blueprints/DamageTypes/DmgType_Instant.DmgType_Instant_C") (== (`self.Daemon`) null) (not (`self.LastShotReleasedSouls`)))
    (set `self.KilledTargetLoc` (`self.K2_GetActorLocation` KilledPawn))
    (set `self.SoulsClaimedPrevious` _soulsclaimed)
    (set `self.SoulsClaimed` (+ _soulsclaimed 1))
    (`self.StealSoulHunterSouls` KilledPawn)
    (if (<= (`self.SoulsClaimed`) (`self.MaxSouls`))
      (`KismetSystemLibrary.K2_ClearTimer` self "LoseSoul" :!label _label) ; Stop timer, if it was active
      (`KismetSystemLibrary.RetriggerableDelay` (`self.LoseSoulsAfter`))
      (`KismetSystemLibrary.K2_SetTimer` self "LoseSoul" (`self.LoseSoulInterval`) true) ; Start losing souls
      (elif (not (< (`KismetMathLibrary.RandomIntegerInRange` 0 100) (* (- (`self.SoulsClaimed`) (`self.MaxSouls`)) 20)))
        (goto _label)))))

(event `self.WeaponPreFireEvent`
  (params (FireMode :type Byte))
  ;[1 1 1] AltFire: release souls
  (if (== FireMode 1)
    (if (> (`self.SoulsClaimed`) 0)
      (for _ (range (+ (`self.SoulsClaimed`) 1))
        (`GameplayStatics.SpawnSoundAttached` "/Game/Sounds/Weapons/SOULHUNTER/SOUL_WAIL.SOUL_WAIL" (`self.Mesh3P`) "None" (0.0 0.0 0.0) (struct) "KeepRelativeOffset" false 1.0 1.0 0.0 null null))
      (`/Engine/EditorBlueprintResources/ActorMacros.Switch Has Authority`
        (:`Authority`
          (`self.SetInstantHitDamage` 1 (`KismetMathLibrary.Round` (* (+ (* (`self.SoulsClaimed`) (`self.SoulsDamageMultiplier`)) 1.0) (`KismetMathLibrary.Conv_IntToDouble` (`self.GetInstantHitDamage` 1)))))
          (set `self.SoulsClaimed` 0)
          (set `self.LastShotReleasedSouls` true))))
    (else
      (set `self.LastShotReleasedSouls` false))))

(event `ClaimedSoulsChanged`
  (bind _soulsclaimedprevious (`self.SoulsClaimedPrevious`))
  (bind _soulsclaimed (`self.SoulsClaimed`))
  ;[0.5 0 0] Material update: souls changed
  (if (> (`self.SoulsClaimed`) (`self.SoulsClaimedPrevious`))
    (`GameplayStatics.SpawnSoundAttached` "/Game/Sounds/Weapons/SOULHUNTER/DEMON_FED_Cue.DEMON_FED_Cue" (`self.Mesh3P`) "None" (0.0 0.0 0.0) (struct) "KeepRelativeOffset" false 1.0 1.0 0.0 null null)
    (bind _returnvalue (`GameplayStatics.SpawnEmitterAttached` "/Game/Weapons/Shotgun/Soul_Capture.Soul_Capture" (`self.GetWeaponMesh`) "Crystal"))
    (`ParticleSystemComponent.SetVectorParameter` _returnvalue "Target" (`self.KilledTargetLoc`))
    (bind (_direction _newtrack_0) (`Timeline|Timeline_0` :!via `PlayFromStart` :!label _label_2)
      (:`Update`
        _)
      (:`Finished`
        _))
    (bind _returnvalue_2 (+ (* _newtrack_0 (`KismetMathLibrary.Abs` (`KismetMathLibrary.Conv_IntToDouble` (- _soulsclaimed _soulsclaimedprevious)))) (`KismetMathLibrary.Conv_IntToDouble` (`KismetMathLibrary.Min` _soulsclaimed _soulsclaimedprevious))))
    (`MaterialInstanceDynamic.SetScalarParameterValue` (`self.Material1P`) "Souls" _returnvalue_2)
    (`MaterialInstanceDynamic.SetScalarParameterValue` (`self.Material3P`) "Souls" _returnvalue_2)
    (else
      (goto _label_2 :!via `ReverseFromEnd`))))

(event `self.SimulateWeaponFireEvent`
  (params (FireMode :type Byte) (InMuzzlePSC :type "ParticleSystemComponent Object Reference"))
  ;[1 1 1] Spawn the three shells after pump
  (`|ExecutionSequence`
    (:`then_0`
      (`KismetSystemLibrary.Delay` 0.75)
      (for _ (range 1 4)
        (`self.SpawnPumpShells` (`SceneComponent.GetSocketTransform` (`self.GetWeaponMesh`) "ShellPumpSocket" "RTS_World"))))
    (:`then_1`
      (if (and (== FireMode 1) (> (`self.SoulsClaimed`) 0))
        (`ParticleSystemComponent.SetTemplate` InMuzzlePSC "/Game/Weapons/Shotgun/Hellfire.Hellfire")))))

(event `self.TracerCreatedEvent`
  (params (ParticleComponent :type "ParticleSystemComponent Object Reference") (FireMode :type Byte) (BounceNum :type Byte) (StartPoint :type "Vector Structure") (EndPoint :type "Vector Structure"))
  (bind _soulsclaimed (`self.SoulsClaimed`))
  (bind _returnvalue (`KismetMathLibrary.Conv_IntToDouble` _soulsclaimed))
  (if (and (== FireMode 1) (> _soulsclaimed 0))
    (`ParticleSystemComponent.SetTemplate` ParticleComponent null)
    (`ParticleSystemComponent.SetVectorParameter` ParticleComponent "SoulsClaimed" (`KismetMathLibrary.MakeVector` _returnvalue _returnvalue _returnvalue))))

(fn `CheckDaemonHealth`
  (if (!= (`self.Daemon`) null)
    (if (<= (`ShooterCharacter.Health` (`self.Daemon`)) 0.0)
      (set `self.Daemon` null)
      (`KismetSystemLibrary.K2_ClearTimer` self "CheckDaemonHealth" :!label _label))
    (else
      (goto _label))))

(fn `LoseSoul`
  (bind _soulsclaimed (`self.SoulsClaimed`))
  (if (== _soulsclaimed 0)
    (`KismetSystemLibrary.K2_ClearTimer` self "LoseSoul" :!label _label)
    (else
      (set `self.SoulsClaimedPrevious` (`self.SoulsClaimed`))
      (set `self.SoulsClaimed` (- _soulsclaimed 1))
      (if (== (`self.SoulsClaimed`) 0)
        (goto _label)))))

(fn `OnRep_SoulsClaimed`
  (`self.ClaimedSoulsChanged`)
  (`self.SetCharacterSpeed` (`self.IsEquipped`)))

(fn `SetCharacterSpeed`
  (params (IsEquipped :type Boolean))
  (bind _returnvalue (`self.GetPawnOwner`))
  (`/Engine/EditorBlueprintResources/StandardMacros.IsValid` _returnvalue
    (:`Is Valid`
      (bind _asshooter_character_movement (cast `ShooterCharacterMovement` (`Character.CharacterMovement` _returnvalue)))
      (if IsEquipped
        (`ShooterCharacterMovement.SetSoulHunterSpeedMod` _asshooter_character_movement (+ (* (`self.SoulsClaimed`) (`self.SpeedIncreasePerSoul`)) 1.0))
        (else
          (`ShooterCharacterMovement.SetSoulHunterSpeedMod` _asshooter_character_movement 1.0))))))

(fn `UserConstructionScript`
  (`parent.UserConstructionScript`))