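; Weapon Blueprint for the Gastraphetes that drives its mesh animation for primary and secondary firing.
; On equip it casts and caches the weapon mesh's AnimBlueprint instance.
; Fire simulation start and stop events toggle that instance's IsFiringPrimary or IsFiringSecondary flag by fire mode.
; The validity check shares the fire-mode branch, so an invalid instance falls through to the secondary path.
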(event `self.WeaponBeingEquippedEvent`
  (bind _returnvalue (`SkeletalMeshComponent.GetAnimInstance` (`self.GetWeaponMesh`)))
  (`/Engine/EditorBlueprintResources/StandardMacros.IsValid` _returnvalue
    (:`Is Valid`
      (bind _assk_gastraphetes_skeleton_anim_blueprint (cast `/Game/Weapons/Gastraphetes/SK_Gastraphetes_Skeleton_AnimBlueprint` _returnvalue))
      (set `self.AnimInst` _assk_gastraphetes_skeleton_anim_blueprint))))

(event `self.SimulateWeaponFireEvent`
  (params (FireMode :type Byte) (InMuzzlePSC :type "ParticleSystemComponent Object Reference"))
  (bind _animinst (`self.AnimInst`))
  (if (and (== FireMode 0) (`KismetSystemLibrary.IsValid` (`self.AnimInst`)))
    (set `/Game/Weapons/Gastraphetes/SK_Gastraphetes_Skeleton_AnimBlueprint.IsFiringPrimary` true _animinst)
    (else
      (set `/Game/Weapons/Gastraphetes/SK_Gastraphetes_Skeleton_AnimBlueprint.IsFiringSecondary` true _animinst))))

(event `self.StopSimulatingWeaponFireEvent`
  (params (FireMode :type Byte))
  (bind _animinst (`self.AnimInst`))
  (if (and (== FireMode 0) (`KismetSystemLibrary.IsValid` (`self.AnimInst`)))
    (set `/Game/Weapons/Gastraphetes/SK_Gastraphetes_Skeleton_AnimBlueprint.IsFiringPrimary` false _animinst)
    (else
      (set `/Game/Weapons/Gastraphetes/SK_Gastraphetes_Skeleton_AnimBlueprint.IsFiringSecondary` false _animinst))))

(fn `UserConstructionScript`
  (`parent.UserConstructionScript`))