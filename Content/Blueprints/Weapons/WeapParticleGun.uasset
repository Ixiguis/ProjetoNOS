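; Particle gun weapon with a primary fire material effect and a charged, wall-penetrating alt-fire beam.
; Charging drives material glow, audio pitch and overload emitters, and stopping or reaching max charge triggers exhaust effects.
; The IsCharging3 RepNotify calls ReleaseCharge, which scales damage, penetration, sound and trail by charge.
; ReleaseCharge back-traces from each forward hit to find exit points, subtracting thickness from remaining penetration and collecting actors to damage.
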(event `self.WeaponBeingEquippedEvent`
  (bind _returnvalue (`self.GetWeaponMesh`))
  (bind _returnvalue_2 (`GameplayStatics.SpawnEmitterAttached` "/Game/Weapons/ParticleGun/P_Overloading.P_Overloading" _returnvalue "exhaust1" (0.0 0.0 0.0) (struct) (1.0 1.0 1.0) "KeepRelativeOffset" false))
  (set `self.OverloadingPSC1` _returnvalue_2)
  (bind _returnvalue_3 (`GameplayStatics.SpawnEmitterAttached` "/Game/Weapons/ParticleGun/P_Overloading.P_Overloading" _returnvalue "exhaust2" (0.0 0.0 0.0) (struct) (1.0 1.0 1.0) "KeepRelativeOffset" false))
  (set `self.OverloadingPSC2` _returnvalue_3)
  (`ActorComponent.Deactivate` (`self.OverloadingPSC1`))
  (`ActorComponent.Deactivate` (`self.OverloadingPSC2`)))

(event `self.WeaponUnequippedEvent`
  (`ActorComponent.K2_DestroyComponent` (`self.OverloadingPSC1`))
  (`ActorComponent.K2_DestroyComponent` (`self.OverloadingPSC2`)))

(event `self.WeaponStartChargeEvent`
  (params (FireMode :type Byte))
  (set `self.IsCharging3` true))

(event `self.WeaponStopChargeEvent`
  (params (FireMode :type Byte) (TotalChargingTime :type "Float (single-precision)"))
  (set `self.IsCharging3` false :!label _label)
  (`self.Start Exhaust Anim`)
  (`ActorComponent.Deactivate` (`self.OverloadingPSC1`))
  (`ActorComponent.Deactivate` (`self.OverloadingPSC2`)))

(event `self.WeaponMaxChargeReachedEvent`
  (params (FireMode :type Byte) (TotalChargingTime :type "Float (single-precision)"))
  (goto _label))

(event `self.ReceiveTick`
  (params (DeltaSeconds :type "Float (single-precision)"))
  (if (`self.IsCharging3`)
    (`self.UpdateMaterials`)
    (if (>= (`self.GetChargingTime`) (`self.MaxChargingTime`))
      (`ActorComponent.Activate` (`self.OverloadingPSC1`) false)
      (`ActorComponent.Activate` (`self.OverloadingPSC2`) false))))

(event `self.UserStartedFiringEvent`
  (params (FireMode :type Byte))
  ;[1 1 1] Primary fire effects
  (if (and (== FireMode 0) (`self.HasEnoughAmmo`))
    (`self.BroadcastSetFiring` true)))

(event `self.UserStoppedFiringEvent`
  (params (FireMode :type Byte))
  ;[1 1 1] Primary fire effects
  (if (and (== FireMode 0) (`self.HasEnoughAmmo`))
    (`self.BroadcastSetFiring` false)))

(event `BroadcastSetFiring`
  (params (IsFiring :type Boolean))
  ;[1 1 1] Primary fire effects
  (`MaterialInstanceDynamic.SetScalarParameterValue` (`self.Material1P`) "Shooting" (`KismetMathLibrary.Conv_BoolToDouble` IsFiring))
  (`MaterialInstanceDynamic.SetScalarParameterValue` (`self.Material3P`) "Shooting" (`KismetMathLibrary.Conv_BoolToDouble` IsFiring)))

(fn `OnRep_IsCharging3`
  (bind _chargeaudio (`self.ChargeAudio`))
  (if (`self.IsCharging3`)
    (`AudioComponent.Play` _chargeaudio 0.0)
    (else
      (`self.ReleaseCharge`)
      (`AudioComponent.Stop` _chargeaudio)
      (`MaterialInstanceDynamic.SetScalarParameterValue` (`self.Material1P`) "Shooting" 0.0)
      (`MaterialInstanceDynamic.SetScalarParameterValue` (`self.Material3P`) "Shooting" 0.0))))

(fn `ReleaseCharge`
  (bind _returnvalue (`self.GetCameraAim`))
  (bind _intensity (`self.Intensity`))
  (bind _returnvalue_2 (`self.GetCameraDamageStartLocation` _returnvalue))
  (bind _returnvalue_3 (+ _returnvalue_2 (* _returnvalue 1000000.0)))
  ;[1 1 1] Determine damage and penetration for this shot
  (set `self.Intensity` (/ (`self.GetChargingTime`) (`self.MaxChargingTime`)))
  (if (> (`self.Intensity`) 0.5)
    (`self.SetFireSound` "/Game/Sounds/Weapons/ParticleGun/PARTICLE_CANNON_SECONDARY_STRONG_Cue.PARTICLE_CANNON_SECONDARY_STRONG_Cue" 1)
    (else
      (`self.SetFireSound` "/Game/Sounds/Weapons/ParticleGun/PARTICLE_CANNON_SECONDARY_WEAK_Cue.PARTICLE_CANNON_SECONDARY_WEAK_Cue" 1)))
  (set `self.CurrentPenetration` (* (`self.AltFireMaxPenetration`) (`self.Intensity`)))
  (set `self.DamageToDeal` (* (`self.AltFireMaxDamage`) (`self.Intensity`)))
  ;[1 1 1] Spawn trail effect
  (bind _returnvalue_4 (`GameplayStatics.SpawnEmitterAtLocation` "/Game/Weapons/ParticleGun/P_Particle_Laser_Sec.P_Particle_Laser_Sec" (.location (`SceneComponent.GetSocketTransform` (`self.GetWeaponMesh`) (`|GetArrayItem` (`self.MuzzleAttachPoint`)) "RTS_World"))))
  (`ParticleSystemComponent.SetVectorParameter` _returnvalue_4 "Intensity" (`KismetMathLibrary.MakeVector` _intensity _intensity _intensity))
  (`ParticleSystemComponent.SetFloatParameter` _returnvalue_4 "Intensity" _intensity)
  (set `self.AltFirePSC` _returnvalue_4)
  ;[1 1 1] Initial trace (from weapon's muzzle)
  (`KismetArrayLibrary.Array_Clear` (`self.DamagedActors`))
  (set `self.FarthestPoint` _returnvalue_3)
  (bind (_outhits _returnvalue_5) (`KismetSystemLibrary.LineTraceMultiForObjects` _returnvalue_2 _returnvalue_3 (`self.TraceObjectTypes`) true (`|MakeArray` (`self.GetPawnOwner`) :!type "Actor Object Reference")))
  (for _array_element _outhits
    (bind (_bblockinghit _binitialoverlap _time _distance _location) (`GameplayStatics.BreakHitResult` _array_element))
    (set `self.FarthestPoint` _location)
    (`self.SpawnImpactEffects` _array_element)
    (bind (_outhits_2 _returnvalue_6) (`KismetSystemLibrary.LineTraceMultiForObjects` (+ (* (`self.GetCameraAim`) (`self.CurrentPenetration`)) _location) _location (`self.TraceObjectTypes`) true))
    (if _returnvalue_6
      (bind _output (`|GetArrayItem` _outhits_2 (- (`KismetArrayLibrary.Array_Length` _outhits_2) 1)))
      (`self.SpawnImpactEffects` _output)
      (bind (_bblockinghit_2 _binitialoverlap_2 _time_2 _distance_2 _location_2 _impactpoint _normal _impactnormal _physmat _hitactor) (`GameplayStatics.BreakHitResult` _output))
      (set `self.FarthestPoint` _location_2)
      (`/Engine/EditorBlueprintResources/StandardMacros.IsValid` _hitactor
        (:`Is Valid`
          (`KismetArrayLibrary.Array_Add` (`self.DamagedActors`) _hitactor)
          (set `self.CurrentPenetration` (`KismetMathLibrary.FMax` (- (`self.CurrentPenetration`) (`KismetMathLibrary.VSize` (- _location _location_2)))))))
      (else
        (set `self.CurrentPenetration` 0.0) ; no hit = trace totally inside wall, not enough penetration
      ))
    (if (not (> (`self.CurrentPenetration`) 0.0))
      (break)))
  (if _returnvalue_5
    (set `self.TrailEndLocation` (`self.FarthestPoint`))
    (else
      (set `self.TrailEndLocation` _returnvalue_3)))
  (`ParticleSystemComponent.SetVectorParameter` (`self.AltFirePSC`) (`self.TrailTargetParam`) (`self.TrailEndLocation`))
  (for _array_element_2 (`self.DamagedActors`)
    (`GameplayStatics.ApplyDamage` _array_element_2 (`self.DamageToDeal`) (`self.GetPawnOwnerController`) self "/Game/Blueprints/DamageTypes/DmgType_Instant.DmgType_Instant_C")))

(fn `Start Exhaust Anim`
  (bind _intensity (`self.Intensity`))
  (bind _intensity_2 (`self.Intensity`))
  (bind _intensity_3 (`self.Intensity`))
  (bind _intensity_4 (`self.Intensity`))
  (bind _mesh1p (`self.Mesh1P`))
  (bind _mesh3p (`self.Mesh3P`))
  (if (not (`KismetSystemLibrary.IsDedicatedServer`))
    (`|ExecutionSequence`
      (:`then_0`
        (if (`self.IsFirstPerson`)
          (bind _assk_particle_gun_skeleton_anim_blueprint (cast `/Game/Weapons/ParticleGun/SK_ParticleGun_Skeleton_AnimBlueprint` (`SkeletalMeshComponent.GetAnimInstance` (`self.Mesh1P`))))
          (`/Game/Weapons/ParticleGun/SK_ParticleGun_Skeleton_AnimBlueprint.Start exhaust` _assk_particle_gun_skeleton_anim_blueprint)
          (bind _returnvalue (`GameplayStatics.SpawnEmitterAttached` "/Game/Weapons/ParticleGun/P_Exhaust.P_Exhaust" _mesh1p "b_rod1"))
          (`ParticleSystemComponent.SetVectorParameter` _returnvalue "Intensity" (`KismetMathLibrary.MakeVector` _intensity_3 _intensity_3 _intensity_3))
          (`ParticleSystemComponent.SetFloatParameter` _returnvalue "Intensity" _intensity_3)
          (bind _returnvalue_2 (`GameplayStatics.SpawnEmitterAttached` "/Game/Weapons/ParticleGun/P_Exhaust.P_Exhaust" _mesh1p "b_rod2"))
          (`ParticleSystemComponent.SetVectorParameter` _returnvalue_2 "Intensity" (`KismetMathLibrary.MakeVector` _intensity _intensity _intensity))
          (`ParticleSystemComponent.SetFloatParameter` _returnvalue_2 "Intensity" _intensity)
          (else
            (bind _assk_particle_gun_skeleton_anim_blueprint_2 (cast `/Game/Weapons/ParticleGun/SK_ParticleGun_Skeleton_AnimBlueprint` (`SkeletalMeshComponent.GetAnimInstance` (`self.Mesh3P`))))
            (`/Game/Weapons/ParticleGun/SK_ParticleGun_Skeleton_AnimBlueprint.Start exhaust` _assk_particle_gun_skeleton_anim_blueprint_2)
            (bind _returnvalue_3 (`GameplayStatics.SpawnEmitterAttached` "/Game/Weapons/ParticleGun/P_Exhaust.P_Exhaust" _mesh3p "b_rod1"))
            (`ParticleSystemComponent.SetVectorParameter` _returnvalue_3 "Intensity" (`KismetMathLibrary.MakeVector` _intensity_4 _intensity_4 _intensity_4))
            (`ParticleSystemComponent.SetFloatParameter` _returnvalue_3 "Intensity" _intensity_4)
            (bind _returnvalue_4 (`GameplayStatics.SpawnEmitterAttached` "/Game/Weapons/ParticleGun/P_Exhaust.P_Exhaust" _mesh3p "b_rod2"))
            (`ParticleSystemComponent.SetVectorParameter` _returnvalue_4 "Intensity" (`KismetMathLibrary.MakeVector` _intensity_2 _intensity_2 _intensity_2))
            (`ParticleSystemComponent.SetFloatParameter` _returnvalue_4 "Intensity" _intensity_2))))
      (:`then_1`
        (`KismetSystemLibrary.K2_SetTimer` null "Stop Exhaust Anim" (- (`self.GetFireRate` 1) 1.0))))))

(fn `Stop Exhaust Anim`
  (if (not (`KismetSystemLibrary.IsDedicatedServer`))
    (bind _assk_particle_gun_skeleton_anim_blueprint (cast `/Game/Weapons/ParticleGun/SK_ParticleGun_Skeleton_AnimBlueprint` (`SkeletalMeshComponent.GetAnimInstance` (`self.Mesh1P`))))
    (`/Game/Weapons/ParticleGun/SK_ParticleGun_Skeleton_AnimBlueprint.Stop Exhaust` _assk_particle_gun_skeleton_anim_blueprint)
    (bind _assk_particle_gun_skeleton_anim_blueprint_2 (cast `/Game/Weapons/ParticleGun/SK_ParticleGun_Skeleton_AnimBlueprint` (`SkeletalMeshComponent.GetAnimInstance` (`self.Mesh3P`))))
    (`/Game/Weapons/ParticleGun/SK_ParticleGun_Skeleton_AnimBlueprint.Stop Exhaust` _assk_particle_gun_skeleton_anim_blueprint_2)))

(fn `UpdateMaterials`
  (`MaterialInstanceDynamic.SetScalarParameterValue` (`self.Material3P`) "Shooting" (`KismetMathLibrary.FMin` (/ (`self.GetChargingTime`) 5.0) 1.0))
  (`MaterialInstanceDynamic.SetScalarParameterValue` (`self.Material1P`) "Shooting" (`KismetMathLibrary.FMin` (/ (`self.GetChargingTime`) 5.0) 1.0))
  (`AudioComponent.SetPitchMultiplier` (`self.ChargeAudio`) (* (+ (/ (`self.GetChargingTime`) (`self.MaxChargingTime`)) 0.4) 1.25)))

(fn `UserConstructionScript`
  (`parent.UserConstructionScript`))