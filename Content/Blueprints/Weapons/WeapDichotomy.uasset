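; Dichotomy weapon whose fire switches between light and shadow depending on whether its wielder stands in sunlight.
; While equipped, a looping timer tests sunlight, swapping primary projectile and sound, secondary trail, and blending a "Sunlit" material parameter.
; Secondary tracers spawn emitters at intervals, each light or shadow by local sunlight.
; Secondary hits deal bonus damage when the character's stored light/shadow value opposes the hit point's lighting, then reset it.
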(event `self.WeaponBeingEquippedEvent`
  ;[1 1 1] Equip/unequip: find Sun and set timers
  (set `self.Sun` (`ShooterBlueprintLibrary.GetSun`))
  (`/Engine/EditorBlueprintResources/StandardMacros.IsValid` (`self.Sun`)
    (:`Is Valid`
      (`KismetSystemLibrary.K2_SetTimer` null "UpdateIsSunlit" 0.2 true)
      (`self.UpdateIsSunlit`))
    (:`Is Not Valid`
      (set `self.IsSunlit` false)))
  (`self.IsSunlitChanged` (`self.IsSunlit`)) ; Ensure an update upon equipping
)

(event `self.WeaponUnequippedEvent`
  ;[1 1 1] Equip/unequip: find Sun and set timers
  (`KismetSystemLibrary.K2_ClearTimer` null "UpdateIsSunlit"))

(event `IsSunlitChanged`
  (params (NewIsSunlit :type Boolean))
  ;[1 1 1] IsSunlit changed
  (set `self.IsSunlit` NewIsSunlit)
  (if NewIsSunlit
    (`self.SetProjectileClass` 0 "/Game/Blueprints/Weapons/Projectiles/ProjDichotomyLightBolt.ProjDichotomyLightBolt_C")
    (`self.SetFireSound` "/Game/Sounds/Weapons/Dichotomy/DICHOTOMY_LIGHT_PRI_Cue.DICHOTOMY_LIGHT_PRI_Cue")
    (`self.SetTrailFX` "/Game/Weapons/Dichotomy/P_LightBeam.P_LightBeam" 1)
    (bind (_direction _newtrack_0) (`Timeline|Interp` :!label _label)
      (:`Update`
        _)
      (:`Finished`
        _))
    (`MaterialInstanceDynamic.SetScalarParameterValue` (`self.Material3P`) "Sunlit" _newtrack_0)
    (`MaterialInstanceDynamic.SetScalarParameterValue` (`self.Material3P_1`) "Sunlit" _newtrack_0)
    (`MaterialInstanceDynamic.SetScalarParameterValue` (`self.Material1P_2`) "Sunlit" _newtrack_0)
    (`MaterialInstanceDynamic.SetScalarParameterValue` (`self.Material3P_2`) "Sunlit" _newtrack_0)
    (`MaterialInstanceDynamic.SetScalarParameterValue` (`self.Material1P_3`) "Sunlit" _newtrack_0)
    (`MaterialInstanceDynamic.SetScalarParameterValue` (`self.Material3P_3`) "Sunlit" _newtrack_0)
    (`MaterialInstanceDynamic.SetScalarParameterValue` (`self.Material1P_4`) "Sunlit" _newtrack_0)
    (`MaterialInstanceDynamic.SetScalarParameterValue` (`self.Material3P_4`) "Sunlit" _newtrack_0)
    (`MaterialInstanceDynamic.SetScalarParameterValue` (`self.Material1P`) "Sunlit" _newtrack_0)
    (`MaterialInstanceDynamic.SetScalarParameterValue` (`self.Material1P_1`) "Sunlit" _newtrack_0)
    (else
      (`self.SetProjectileClass` 0 "/Game/Blueprints/Weapons/Projectiles/ProjDichotomyShadowBolt.ProjDichotomyShadowBolt_C")
      (`self.SetFireSound` "/Game/Sounds/Weapons/Dichotomy/DICHOTOMY_SHADOW_PRI_Cue.DICHOTOMY_SHADOW_PRI_Cue")
      (`self.SetTrailFX` "/Game/Weapons/Dichotomy/P_ShadowBeam.P_ShadowBeam" 1)
      (goto _label :!via `Reverse`))))

(event `self.TracerCreatedEvent`
  (params (ParticleComponent :type "ParticleSystemComponent Object Reference") (FireMode :type Byte) (BounceNum :type Byte) (StartPoint :type "Vector Structure") (EndPoint :type "Vector Structure"))
  (bind _returnvalue (- (`self.ShotTarget`) (`self.ShotStart`)))
  (bind _returnvalue_2 (`KismetMathLibrary.Normal` _returnvalue))
  ;[1 1 1] Secondary fire: update trail effects along the tracer
  (`/Engine/EditorBlueprintResources/StandardMacros.IsValid` (`self.Sun`)
    (:`Is Valid`
      (set `self.ShotStart` StartPoint)
      (set `self.ShotTarget` EndPoint)
      (set `self.ShotLength` (`KismetMathLibrary.VSize` _returnvalue))
      (set `self.ShotDirection` _returnvalue_2)
      (set `self.ShotRotation` (`KismetMathLibrary.Conv_VectorToRotator` _returnvalue_2))
      (for _index (range 1 (+ (`KismetMathLibrary.Min` (`KismetMathLibrary.FCeil` (/ (`self.ShotLength`) (`self.TrailSpacing`))) 100) 1))
        (bind _returnvalue_3 (+ (`self.ShotStart`) (* (`self.ShotDirection`) (* _index (`self.TrailSpacing`)))))
        (`GameplayStatics.SpawnEmitterAtLocation` (select `bool` (`ShooterBlueprintLibrary.LocationIsSunlit` _returnvalue_3 (`|MakeArray` self (`self.GetInstigator`) :!type "Actor Object Reference") (`self.Sun`)) :`false` "/Game/Weapons/Dichotomy/Effects/P_DichotomyAltFireBeam_Shadow.P_DichotomyAltFireBeam_Shadow" :`true` "/Game/Weapons/Dichotomy/Effects/P_DichotomyAltFireBeam_Light.P_DichotomyAltFireBeam_Light" :!type "ParticleSystem Object Reference") _returnvalue_3 (`self.ShotRotation`))))))

(event `self.WeaponDealtDamageEvent`
  (params (HitResult :type "HitResult Structure") (DamageInfo :type "PointDamageEvent Structure") (ShootDir :type "Vector Structure") (FireMode :type Byte) (BounceNumber :type Byte))
  (bind (_bblockinghit _binitialoverlap _time _distance _location _impactpoint _normal _impactnormal _physmat _hitactor) (`GameplayStatics.BreakHitResult` HitResult))
  (bind _asshooter_character_bp (cast `/Game/Blueprints/Pawns/ShooterCharacter_BP` _hitactor))
  (`GameplayStatics.ApplyDamage` _asshooter_character_bp (* (`KismetMathLibrary.FMax` (- (`KismetMathLibrary.Abs` (- (`/Game/Blueprints/Pawns/ShooterCharacter_BP.DichotomyLightOrShadow` _asshooter_character_bp) (`KismetMathLibrary.MapRangeUnclamped` (`KismetMathLibrary.Conv_BoolToDouble` (`ShooterBlueprintLibrary.LocationIsSunlit` _location (`|MakeArray` _asshooter_character_bp (`self.GetInstigator`) self :!type "Actor Object Reference") (`self.Sun`))) 0.0 1.0 -1.0 1.0))) 1.0)) (`self.SecBonusDamage`)) (`self.GetPawnOwnerController`) self "/Game/Blueprints/DamageTypes/DichotomySecondaryShot.DichotomySecondaryShot_C")
  (`/Game/Blueprints/Pawns/ShooterCharacter_BP.DichotomyResetLight` _asshooter_character_bp))

(fn `UpdateIsSunlit`
  (bind _returnvalue (`self.GetPawnOwner`))
  (bind _issunlit (`self.IsSunlit`))
  (`/Engine/EditorBlueprintResources/StandardMacros.IsValid` _returnvalue
    (:`Is Valid`
      (set `self.IsSunlitTestLocation` (`self.K2_GetActorLocation` _returnvalue)))
    (:`Is Not Valid`
      (set `self.IsSunlitTestLocation` (`self.GetMuzzleLocation`))))
  (if (`ShooterBlueprintLibrary.LocationIsSunlit` (`self.IsSunlitTestLocation`) (`|MakeArray` self (`self.GetInstigator`) :!type "Actor Object Reference") (`self.Sun`))
    (if (not _issunlit)
      (`self.IsSunlitChanged` true))
    (elif _issunlit
      (`self.IsSunlitChanged` false))))

(fn `UserConstructionScript`
  (`parent.UserConstructionScript`)
  (bind _returnvalue (`PrimitiveComponent.CreateDynamicMaterialInstance` (`self.Mesh1P`) 1 null "None"))
  (set `self.Material1P_1` _returnvalue)
  (bind _returnvalue_2 (`PrimitiveComponent.CreateDynamicMaterialInstance` (`self.Mesh3P`) 1 null "None"))
  (set `self.Material3P_1` _returnvalue_2)
  (bind _returnvalue_3 (`PrimitiveComponent.CreateDynamicMaterialInstance` (`self.Mesh1P`) 2 null "None"))
  (set `self.Material1P_2` _returnvalue_3)
  (bind _returnvalue_4 (`PrimitiveComponent.CreateDynamicMaterialInstance` (`self.Mesh3P`) 2 null "None"))
  (set `self.Material3P_2` _returnvalue_4)
  (bind _returnvalue_5 (`PrimitiveComponent.CreateDynamicMaterialInstance` (`self.Mesh1P`) 3 null "None"))
  (set `self.Material1P_3` _returnvalue_5)
  (bind _returnvalue_6 (`PrimitiveComponent.CreateDynamicMaterialInstance` (`self.Mesh3P`) 3 null "None"))
  (set `self.Material3P_3` _returnvalue_6)
  (bind _returnvalue_7 (`PrimitiveComponent.CreateDynamicMaterialInstance` (`self.Mesh1P`) 4 null "None"))
  (set `self.Material1P_4` _returnvalue_7)
  (bind _returnvalue_8 (`PrimitiveComponent.CreateDynamicMaterialInstance` (`self.Mesh3P`) 4 null "None"))
  (set `self.Material3P_4` _returnvalue_8))