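; Impaler sniper weapon with a variable-zoom scope and the ability to impale killed characters on nearby surfaces.
; Custom fire toggles the scope for the local player, enabling zoom inputs that drive a timeline to step zoom between clamped limits.
; Unequipping resets zoom and disables that input.
; CheckImpalement traces from the victim along the shot direction and, if a surface is within range, spawns a ProjImpaler at the hit carrying the victim.
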(event `self.StartCustomFire`
  (params (FireMode :type Byte))
  (bind _pc (`self.PC`))
  ;[1 1 1] Zoom toggle
  (if (`Pawn.IsLocallyControlled` (`self.GetPawnOwner`))
    (bind _asshooter_player_controller (cast `ShooterPlayerController` (`self.GetPawnOwnerController`)))
    (set `self.PC` _asshooter_player_controller)
    (set `self.IsZooming` (not (`self.IsZooming`)))
    (if (`self.IsZooming`)
      (set `self.CurrentZoomPercent` (`self.MinZoomPercent`))
      (`self.EnableInput` _pc)
      (`GameplayStatics.PlaySoundAtLocation` "/Game/Sounds/Weapons/Impaler/IMPALER_SCOPE_ON_Cue.IMPALER_SCOPE_ON_Cue" (0.0 0.0 0.0) (struct) 1.0 1.0 0.0 null null null)
      (else
        (set `self.CurrentZoomPercent` 0.0)
        (`self.DisableInput` _pc)
        (`GameplayStatics.PlaySoundAtLocation` "/Game/Sounds/Weapons/Impaler/IMPALER_SCOPE_OUT_Cue.IMPALER_SCOPE_OUT_Cue" (0.0 0.0 0.0) (struct) 1.0 1.0 0.0 null null null)))
    (`ShooterPlayerController.SetZoomLevel` (`self.PC`) (`self.CurrentZoomPercent`) (`self.MinFOV`) :!label _label)))

(event `self.WeaponUnequippedEvent`
  ;[1 1 1] Zoom toggle
  (bind _asshooter_player_controller (cast `ShooterPlayerController` (`self.GetPawnOwnerController`)))
  (set `self.PC` _asshooter_player_controller)
  (set `self.CurrentZoomPercent` 0.0)
  (set `self.IsZooming` false)
  (`self.DisableInput` (`self.PC`))
  (goto _label))

(event `InputAction|SniperZoomIn`
  (params (Key :type "Key Structure"))
  (bind _currentzoompercent (`self.CurrentZoomPercent`))
  ;[1 1 1] Zoom in/out
  (:`Pressed`
    (if (`self.IsZooming`)
      (set `self.Increment` (`self.ZoomIncrement`))
      (if (and (> _currentzoompercent (`self.MinZoomPercent`)) (< _currentzoompercent 1.0)) :!label _label_2
        (`GameplayStatics.PlaySoundAtLocation` "/Game/Sounds/Weapons/Impaler/IMPALER_CHANGE_ZOOM_Cue.IMPALER_CHANGE_ZOOM_Cue" (0.0 0.0 0.0) (struct) 1.0 1.0 0.0 null null null)
        (bind (_direction _zoom) (`Timeline|Zoom` :!via `PlayFromStart` :!label _label_3)
          (:`Update`
            _)
          (:`Finished`
            _))
        (set `self.CurrentZoomPercent` (`KismetMathLibrary.FClamp` (+ (`self.CurrentZoomPercent`) (* _zoom (`self.Increment`))) (`self.MinZoomPercent`)))
        (`ShooterPlayerController.SetZoomLevel` (`self.PC`) (`self.CurrentZoomPercent`) (`self.MinFOV`))
        (else
          (goto _label_3 :!via `PlayFromStart`))))))

(event `InputAction|SniperZoomOut`
  (params (Key :type "Key Structure"))
  ;[1 1 1] Zoom in/out
  (:`Pressed`
    (if (`self.IsZooming`)
      (set `self.Increment` (- 0.0 (`self.ZoomIncrement`)))
      (goto _label_2))))

(event `InputAction|NextWeapon`
  (params (Key :type "Key Structure"))
  ;[1 1 1] Prevent SniperZoomIn/Out bindings from working... @todo: should be GetKeyBind(SniperZoomIn)
)

(event `InputAction|PrevWeapon`
  (params (Key :type "Key Structure"))
  ;[1 1 1] Prevent SniperZoomIn/Out bindings from working... @todo: should be GetKeyBind(SniperZoomIn)
)

(fn `CheckImpalement`
  (params (TestCharacter :type "ShooterCharacter Object Reference") (HitInfo :type "HitResult Structure") (ShotDirection :type "Vector Structure"))
  (returns (ProjImpaler :type "ShooterProjectile Object Reference") (Impaled :type Boolean))
  (bind _returnvalue (`self.K2_GetActorLocation` (`self.KilledPawn`)))
  (set `self.ShotDirection` ShotDirection)
  (set `self.KilledPawn` TestCharacter)
  (bind (_outhit _returnvalue_2) (`KismetSystemLibrary.LineTraceSingleForObjects` _returnvalue (+ _returnvalue (* (`self.ShotDirection`) (`self.ImpaleMaxDistance`))) (`self.ImpaleSurfaces`) false (`|MakeArray` (`self.KilledPawn`) :!type "Actor Object Reference"))) ; Check if pawn is nearby a wall
  (if _returnvalue_2
    (bind _returnvalue_3 (`|SpawnActorFromClass` "/Game/Blueprints/Weapons/Projectiles/ProjImpaler.ProjImpaler_C" (`KismetMathLibrary.MakeTransform` (`.Location` (`GameplayStatics.BreakHitResult` HitInfo)) (`KismetMathLibrary.Conv_VectorToRotator` ShotDirection)) "AlwaysSpawn" "OverrideRootScale" null null))
    (set `/Game/Blueprints/Weapons/Projectiles/ProjImpaler.ImpaledCharacter` TestCharacter _returnvalue_3))
  (return _returnvalue_3 _returnvalue_2))

(fn `UserConstructionScript`
  (`parent.UserConstructionScript`))