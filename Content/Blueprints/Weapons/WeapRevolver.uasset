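; Revolver weapon whose primary fire plants explosive bullets at hit points and whose alt-fire detonates them all.
; The server spawns bullets from instant-hit events, or from damage events for damageable actors to avoid client-server position mismatch.
; Bullets attach to living characters and movable meshes but explode on dying pawns.
; A tracked array detonates the oldest at the limit, replaces near-simultaneous spawns and is cleared on weapon destruction.
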(event `self.ReceiveDestroyed`
  (`self.DestroyAllBullets`))

(event `self.WeaponInstantHitEvent`
  (params (FireMode :type Byte) (Impact :type "HitResult Structure") (InstigatorCharacter :type "ShooterCharacter Object Reference"))
  (bind (_bblockinghit _binitialoverlap _time _distance _location _impactpoint _normal _impactnormal _physmat _hitactor _hitcomponent) (`GameplayStatics.BreakHitResult` Impact))
  (bind _spawnedbullet (`self.SpawnedBullet`))
  (if (== FireMode 0)
    (`self.Play animation`)
    (`/Engine/EditorBlueprintResources/ActorMacros.Switch Has Authority`
      (:`Authority`
        (set `self.HitLoc` _location)
        (set `self.HitNormal` _impactnormal)
        (if (== _hitactor null)
          (`self.SpawnProjectile` :!label _label)
          (elif (not (`Actor.bCanBeDamaged` _hitactor))
            (set `self.ActorHit` _hitactor)
            (set `self.ComponentHit` _hitcomponent)
            (`|ExecutionSequence` :!label _label_2
              (:`then_0`
                (goto _label))
              (:`then_1`
                (bind _asshooter_character_bp (cast `/Game/Blueprints/Pawns/ShooterCharacter_BP` (`self.ActorHit`)) ; Hit a character?
                  (:`then`
                    (if (`ShooterCharacter.bIsDying` _asshooter_character_bp)
                      (`ShooterProjectile.ExplodeProjectile` _spawnedbullet) ; Explode immediately if pawn is dead/dying
                      (else
                        (`self.K2_AttachRootComponentTo` _spawnedbullet (`Character.Mesh` _asshooter_character_bp) (`self.BoneHit`) "KeepWorldPosition" true) ; Attach to pawn if he's alive
                      )))
                  (:`CastFailed`
                    (bind _asmesh_component (cast `MeshComponent` (`self.ComponentHit`))) ; Hit another dynamic actor?
                    (if (`|EnumEquality` (`SceneComponent.Mobility` _asmesh_component) "Movable")
                      (`self.K2_AttachRootComponentTo` (`self.SpawnedBullet`) _asmesh_component "None" "KeepWorldPosition" true))))))))))))

(event `self.WeaponDealtDamageEvent`
  (params (HitResult :type "HitResult Structure") (DamageInfo :type "PointDamageEvent Structure") (ShootDir :type "Vector Structure") (FireMode :type Byte) (BounceNumber :type Byte))
  (bind (_bblockinghit _binitialoverlap _time _distance _location _impactpoint _normal _impactnormal _physmat _hitactor _hitcomponent _hitbonename) (`GameplayStatics.BreakHitResult` HitResult))
  (set `self.HitLoc` _impactpoint)
  (set `self.HitNormal` _impactnormal)
  (set `self.ActorHit` _hitactor)
  (set `self.ComponentHit` _hitcomponent)
  (set `self.BoneHit` _hitbonename)
  (goto _label_2))

(event `self.WeaponPreFireEvent`
  (params (FireMode :type Byte))
  ;[1 1 1] AltFire: explode all bullets
  (if (== FireMode 1)
    (`self.ExplodeAllBullets`)))

(fn `DespawnProjectile`
  (params (Projectile :type "/Game/Blueprints/Weapons/Projectiles/ProjRevolverExplosive Object Reference"))
  (bind _spawnedbullets (`self.SpawnedBullets`))
  (bind _returnvalue (`KismetArrayLibrary.Array_RemoveItem` _spawnedbullets Projectile))
  (if _returnvalue
    (`self.K2_DestroyActor` Projectile)
    (set `self.NumSpawnedBullets` (`KismetMathLibrary.Conv_IntToByte` (`KismetArrayLibrary.Array_Length` _spawnedbullets)))))

(fn `DestroyAllBullets`
  (bind _spawnedbullets (`self.SpawnedBullets`))
  (`/Engine/EditorBlueprintResources/ActorMacros.Switch Has Authority`
    (:`Authority`
      (if (> (`KismetArrayLibrary.Array_Length` _spawnedbullets) 0)
        (for _array_element _spawnedbullets
          (`self.K2_DestroyActor` _array_element))
        (`KismetArrayLibrary.Array_Clear` _spawnedbullets)
        (set `self.NumSpawnedBullets` (`KismetMathLibrary.Conv_IntToByte` (`KismetArrayLibrary.Array_Length` _spawnedbullets)))))))

(fn `ExplodeAllBullets`
  (bind _spawnedbullets (`self.SpawnedBullets`))
  (for _array_element _spawnedbullets
    (`/Engine/EditorBlueprintResources/StandardMacros.IsValid` _array_element
      (:`Is Valid`
        (`ShooterProjectile.ExplodeProjectile` _array_element))))
  (`KismetArrayLibrary.Array_Clear` _spawnedbullets)
  (set `self.NumSpawnedBullets` 0))

(fn `RemoveBullet`
  (params (Bullet :type "ShooterProjectile Object Reference"))
  (bind _spawnedbullets (`self.SpawnedBullets`))
  (`/Engine/EditorBlueprintResources/ActorMacros.Switch Has Authority`
    (:`Authority`
      (bind _returnvalue (`KismetArrayLibrary.Array_RemoveItem` _spawnedbullets Bullet))
      (if _returnvalue
        (set `self.NumSpawnedBullets` (`KismetMathLibrary.Conv_IntToByte` (`KismetArrayLibrary.Array_Length` _spawnedbullets)))))))

(fn `SpawnProjectile`
  (bind _spawnedbullets (`self.SpawnedBullets`))
  (if (< (- (`KismetSystemLibrary.GetGameTimeInSeconds`) (`self.LastBulletSpawnTime`)) 0.1)
    (bind _asproj_revolver_explosive (cast `/Game/Blueprints/Weapons/Projectiles/ProjRevolverExplosive` (`self.SpawnedBullet`)))
    (`self.DespawnProjectile` _asproj_revolver_explosive) ; If spawned 2+ bullets at the same time, despawn the first one
  )
  (set `self.LastBulletSpawnTime` (`KismetSystemLibrary.GetGameTimeInSeconds`))
  (bind _returnvalue (`|SpawnActorFromClass` "/Game/Blueprints/Weapons/Projectiles/ProjRevolverExplosive.ProjRevolverExplosive_C" (`KismetMathLibrary.Conv_VectorToTransform` (`self.HitLoc`)) "Undefined" "OverrideRootScale" null null))
  (`self.K2_SetActorRotation` _returnvalue (`KismetMathLibrary.Conv_VectorToRotator` (- (0.0 0.0 0.0) (`self.HitNormal`))) false)
  (bind _asshooter_projectile (cast `ShooterProjectile` _returnvalue))
  (set `self.SpawnedBullet` _asshooter_projectile)
  (`ShooterProjectile.SetInstigator` _asshooter_projectile (`self.GetPawnOwner`))
  (bind _returnvalue_2 (`KismetArrayLibrary.Array_Add` (`self.SpawnedBullets`) (`self.SpawnedBullet`)))
  (if (>= _returnvalue_2 (`self.ExplosivesLimit`))
    (`ShooterProjectile.ExplodeProjectile` (`|GetArrayItem` (`self.SpawnedBullets`)))
    (`KismetArrayLibrary.Array_Remove` _spawnedbullets))
  (set `self.NumSpawnedBullets` (`KismetMathLibrary.Conv_IntToByte` (`KismetArrayLibrary.Array_Length` _spawnedbullets))))

(fn `UserConstructionScript`
  (`parent.UserConstructionScript`))