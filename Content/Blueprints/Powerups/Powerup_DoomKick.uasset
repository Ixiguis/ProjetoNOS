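; Doom Kick powerup that boosts the shooter character's kick damage, kick impulse and movement speed while active.
; Activation writes the boosted values to the pawn and attaches foot particle emitters to the first-person body mesh or the third-person mesh.
; Deactivation restores kick stats from the pawn class's default object, resets the speed modifier and deactivates both emitters.
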(event `self.ActivatedEvent`
  (bind _asshooter_character_bp (cast `/Game/Blueprints/Pawns/ShooterCharacter_BP` (`self.MyPawn`)))
  (set `/Game/Blueprints/Pawns/ShooterCharacter_BP.KickDamage` (`self.BoostedKickDamage`) _asshooter_character_bp)
  (set `/Game/Blueprints/Pawns/ShooterCharacter_BP.KickImpulseStrength` (`self.BoostedKickImpulseStrength`) _asshooter_character_bp)
  (bind _asshooter_character_movement (cast `ShooterCharacterMovement` (`Character.CharacterMovement` _asshooter_character_bp))
    (:`then`
      (`ShooterCharacterMovement.SetPowerupSpeedMod` _asshooter_character_movement (`self.SpeedModifierBoost`)))
    (:`CastFailed`
      _))
  (`self.AttachEffects`))

(event `self.DeactivatedEvent`
  (bind _mypawn (`self.MyPawn`))
  (bind _asshooter_character_bp (cast `/Game/Blueprints/Pawns/ShooterCharacter_BP` (`ShooterBlueprintLibrary.GetDefaultObject` _mypawn))) ; defaults
  (bind _asshooter_character_bp_2 (cast `/Game/Blueprints/Pawns/ShooterCharacter_BP` _mypawn)) ; to be changed
  (set `/Game/Blueprints/Pawns/ShooterCharacter_BP.KickDamage` (`/Game/Blueprints/Pawns/ShooterCharacter_BP.KickDamage` _asshooter_character_bp) _asshooter_character_bp_2)
  (set `/Game/Blueprints/Pawns/ShooterCharacter_BP.KickImpulseStrength` (`/Game/Blueprints/Pawns/ShooterCharacter_BP.KickImpulseStrength` _asshooter_character_bp) _asshooter_character_bp_2)
  (bind _asshooter_character_movement (cast `ShooterCharacterMovement` (`Character.CharacterMovement` _asshooter_character_bp_2))
    (:`then`
      (`ShooterCharacterMovement.SetPowerupSpeedMod` _asshooter_character_movement 1.0))
    (:`CastFailed`
      _))
  (`self.RemoveEffects`))

(event `AttachEffects`
  (bind _usemesh (`self.UseMesh`))
  (bind _mypawn (`self.MyPawn`))
  (if (`ShooterCharacter.IsFirstPerson` _mypawn)
    (bind _asplayer_pawn (cast `/Game/Blueprints/Pawns/PlayerPawn` _mypawn)
      (:`then`
        (set `self.UseMesh` (`/Game/Blueprints/Pawns/PlayerPawn.Mesh1PBody` _asplayer_pawn)))
      (:`CastFailed`
        (set `self.UseMesh` (`ShooterCharacter.GetPawnMesh3P` _mypawn) :!label _label)))
    (else
      (goto _label)))
  (bind _returnvalue (`GameplayStatics.SpawnEmitterAttached` "/Game/Effects/Particles/Gameplay/Items/P_DoomKick.P_DoomKick" _usemesh "b_LeftFoot"))
  (set `self.LeftFootPSC` _returnvalue)
  (bind _returnvalue_2 (`GameplayStatics.SpawnEmitterAttached` "/Game/Effects/Particles/Gameplay/Items/P_DoomKick.P_DoomKick" _usemesh "b_RightFoot" (0.0 0.0 0.0)))
  (set `self.RightFootPSC` _returnvalue_2))

(event `RemoveEffects`
  (`ActorComponent.Deactivate` (`self.RightFootPSC`))
  (`ActorComponent.Deactivate` (`self.LeftFootPSC`))
  (set `self.LeftFootPSC` null)
  (set `self.RightFootPSC` null))

(fn `UserConstructionScript`
  (`parent.UserConstructionScript`))