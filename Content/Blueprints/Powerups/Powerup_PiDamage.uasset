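; Pi damage powerup that boosts the holding pawn's damage scale while active.
; Activation sets DamageScale to pi and deactivation resets it to normal.
; It also attaches a particle emitter to both weapon points, choosing the first- or third-person mesh by view, and deactivates and clears those emitters when the powerup ends.
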(event `self.ActivatedEvent`
  (bind _mypawn (`self.MyPawn`))
  (if (!= _mypawn null)
    (set `ShooterCharacter.DamageScale` (`KismetMathLibrary.MultiplyByPi` 1.0) _mypawn)
    (`self.AttachEffects`)))

(event `self.DeactivatedEvent`
  (bind _mypawn (`self.MyPawn`))
  (if (!= _mypawn null)
    (set `ShooterCharacter.DamageScale` 1.0 _mypawn)
    (`self.RemoveEffects`)))

(event `AttachEffects`
  (bind _usemesh (`self.UseMesh`))
  (bind _mypawn (`self.MyPawn`))
  (if (`ShooterCharacter.IsFirstPerson` _mypawn)
    (set `self.UseMesh` (`ShooterCharacter.GetPawnMesh1P` _mypawn))
    (else
      (set `self.UseMesh` (`ShooterCharacter.GetPawnMesh3P` _mypawn))))
  (bind _returnvalue (`GameplayStatics.SpawnEmitterAttached` "/Game/Effects/Particles/Gameplay/Items/P_PiDamage.P_PiDamage" _usemesh "WeaponPoint"))
  (set `self.RightHandPSC` _returnvalue)
  (bind _returnvalue_2 (`GameplayStatics.SpawnEmitterAttached` "/Game/Effects/Particles/Gameplay/Items/P_PiDamage.P_PiDamage" _usemesh "LeftWeaponPoint"))
  (set `self.LeftHandPSC` _returnvalue_2))

(event `RemoveEffects`
  (`ActorComponent.Deactivate` (`self.LeftHandPSC`))
  (`ActorComponent.Deactivate` (`self.RightHandPSC`))
  (set `self.RightHandPSC` null)
  (set `self.LeftHandPSC` null))

(fn `UserConstructionScript`
  (`parent.UserConstructionScript`))